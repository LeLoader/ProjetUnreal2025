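; AC_SerpadentMove is an actor component that moves its owner, presumably the Serpadent, along a navigation spline.
; MoveAlongSpline places the owner at the offset distance on the spline, without sweeping.
; Passing spline point 2 resets the travelled distance and reports reaching the next point, flagging whether it is the last.
; As written, the distance increment is always zero because DeltaSeconds and Speed are unused.
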(event EventBeginPlay
  (|CallParentFunction) ; This node is disabled and will not be called.\nDrag off pins to build functionality.
)

(event EventTick
  (params (DeltaSeconds :type Float%20%28single-precision%29))
  (|CallParentFunction DeltaSeconds) ; This node is disabled and will not be called.\nDrag off pins to build functionality.
)

(fn MoveAlongSpline
  (params (DeltaSeconds :type Float%20%28double-precision%29) (Speed :type Float%20%28double-precision%29))
  (bind _distance (CallFunction|GetDistancewithOffset))
  (bind _navigationspline (Variables|Default|GetNavigationSpline))
  (Variables|Default|SetActualDistanceAlongSpline (+ (* 0.0 (* 0.0 1e+02)) (Variables|Default|GetActualDistanceAlongSpline)))
  (Transformation|SetActorLocation (Components|GetOwner) (Spline|GetLocationatDistanceAlongSpline _navigationspline _distance "World") false false)
  (if (<= (Spline|GetDistanceAlongSplineatSplinePoint _navigationspline 2) _distance)
    (Variables|Default|SetActualDistanceAlongSpline 0.0)
    (return true (<= (Spline|GetDistanceAlongSplineatSplinePoint _navigationspline (- (Spline|GetNumberOfSplinePoints _navigationspline) 1)) _distance))
    (else
      (return false false))))