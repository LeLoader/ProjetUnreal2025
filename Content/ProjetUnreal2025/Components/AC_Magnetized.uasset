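; Actor component that magnetizes an actor to a named socket on a skeletal mesh.
; Each tick it interpolates the actor's root transform toward the socket's world transform at a set magnetize speed, without sweeping.
; Once the interpolated location is within a small distance of the socket, it attaches the actor with snap-to-target rules and destroys itself.
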(event EventTick
  (params (DeltaSeconds :type Float%20%28single-precision%29))
  (bind _magnetizespeed (Variables|Default|GetMagnetizeSpeed))
  (bind _actor (Variables|Default|GetActor))
  (bind _skeletalmesh (Variables|Default|GetSkeletalMesh))
  (bind _name (Variables|Default|GetName))
  (bind _returnvalue (Transformation|GetSocketTransform _skeletalmesh _name "RTS_World"))
  (bind _returnvalue_2 (Transformation|GetActorTransform _actor))
  (bind _returnvalue_3 (Class|KismetMathLibrary|TInterpto _returnvalue_2 _returnvalue DeltaSeconds _magnetizespeed))
  (if (<= (Math|Vector|Distance(Vector) (.Location (Math|Transform|BreakTransform _returnvalue_3)) (.Location (Math|Transform|BreakTransform _returnvalue))) 1e+01)
    (Transformation|AttachComponentToComponent (Variables|Default|GetActor) (Variables|Default|GetSkeletalMesh) (Variables|Default|GetName) "SnapToTarget" "SnapToTarget" "SnapToTarget" true)
    (Components|DestroyComponent)
    (else
      (Transformation|SetWorldTransform (Variables|/Script/Engine.Actor|GetRootComponent (Variables|Default|GetActor)) _returnvalue_3 false false))))