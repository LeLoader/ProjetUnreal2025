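; Fish movement component that moves its owning actor along a navigation spline whenever MoveAlongSpline is called.
; Travel distance grows with speed and delta time, offset to start at spline point 1.
; Optional rotation follows the spline tangent, using the actor's world location as the up axis (radial from the origin).
; Reaching point 2 resets the distance and returns next-point and last-point flags to the caller.
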(event EventBeginPlay)

(event EventTick
  (params (DeltaSeconds :type Float%20%28single-precision%29)))

(fn MoveAlongSpline
  (params (DeltaSeconds :type Float%20%28double-precision%29) (Speed :type Float%20%28double-precision%29) (RotateFish :type Boolean))
  (bind _returnvalue (Components|GetOwner))
  (bind _distance (CallFunction|GetDistancewithOffset))
  (bind _navigationspline (Variables|Default|GetNavigationSpline))
  (Variables|Default|SetActualDistanceAlongSpline (+ (* DeltaSeconds (* Speed 1e+02)) (Variables|Default|GetActualDistanceAlongSpline)))
  (Transformation|SetActorLocation _returnvalue (Spline|GetLocationatDistanceAlongSpline _navigationspline _distance "World") false false)
  (if RotateFish
    (Transformation|SetActorRotation _returnvalue (Math|Rotator|MakeRotfromZX (Transformation|GetActorLocation _returnvalue) (Spline|GetTangentatDistanceAlongSpline _navigationspline _distance "Local"))))
  (if (<= (Spline|GetDistanceAlongSplineatSplinePoint _navigationspline 2) _distance)
    (Variables|Default|SetActualDistanceAlongSpline 0.0)
    (return true (<= (Spline|GetDistanceAlongSplineatSplinePoint _navigationspline (- (Spline|GetNumberOfSplinePoints _navigationspline) 1)) _distance))
    (else
      (return false false))))

(fn ResetDistance
  (Variables|Default|SetActualDistanceAlongSpline 0.0))

(fn GetDistancewithOffset
  (return (+ (Variables|Default|GetActualDistanceAlongSpline) (Spline|GetDistanceAlongSplineatSplinePoint (Variables|Default|GetNavigationSpline) 1))))