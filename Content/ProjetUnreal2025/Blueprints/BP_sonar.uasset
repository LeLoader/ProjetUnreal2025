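; BP_sonar is an interactable sonar that plays a start sound and sweeps for objects along its forward vector when Interact fires.
; It caches GI_Fish on BeginPlay and uses the distance to that instance's PlanetCenter as the sweep length.
; The sweep is a multi-sphere object trace on one custom object type with persistent debug drawing.
; The trace hits are not used yet.
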(event EventBeginPlay
  (bind _asgi_fish (Utilities|Casting|CastToGI_Fish (Game|GetGameInstance)))
  (Variables|Default|SetGI%20Fish _asgi_fish))

(event EventInteract
  (params (LeftClick :type Boolean) (IsHoldingSomething :type Boolean) (Player :type BP%20Fisherman%20Object%20Reference))
  (bind _returnvalue (Transformation|GetActorLocation))
  (Development|PrintString "Interact")
  (Variables|Default|SetSonarLength (Math|Vector|Distance(Vector) (Transformation|GetActorLocation) (Variables|/Game/ProjetUnreal2025/Blueprints/Global/GI_Fish.GI_Fish_C|GetPlanetCenter (Variables|Default|GetGI%20Fish))))
  (Audio|PlaySound2D (Variables|Default|GetStartSonarSound) 1.0 1.0 0.0 0 0)
  (Collision|MultiSphereTraceForObjects _returnvalue (+ _returnvalue (* (Transformation|GetActorForwardVector) (Variables|Default|GetSonarLength))) (Variables|Default|GetSonarRadius) (Utilities|Array|MakeArray "ObjectTypeQuery9") false 0 "Persistent"))

(fn ConstructionScript)