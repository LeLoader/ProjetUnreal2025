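; BP_Planet is the planet actor that anchors the boat's spline and reacts to thrown or moving bait.
; On BeginPlay it spawns a BP_Boat, registers its center, boat and spline in GI_Fish, and places the boat on the spline.
; Its GravityZone slows entering BP_Bait and its Sphere destroys bait on contact.
; A helper returns the center-relative surface offset toward a given point, derived from actor scale.
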(event OnComponentBeginOverlap(GravityZone)
  (params (OverlappedComponent :type Primitive%20Component%20Object%20Reference) (OtherActor :type Actor%20Object%20Reference) (OtherComp :type Primitive%20Component%20Object%20Reference) (OtherBodyIndex :type Integer) (bFromSweep :type Boolean) (SweepResult :type Hit%20Result%20Structure%20%28by%20ref%29))
  ;[0.15 0.15 0.15 0.5] Slow Bait when entering Gravity Zone
  (bind _asbp_bait (Utilities|Casting|CastToBP_Bait OtherActor))
  (Default|CEReduceSpeed _asbp_bait))

(event OnComponentBeginOverlap(Sphere)
  (params (OverlappedComponent :type Primitive%20Component%20Object%20Reference) (OtherActor :type Actor%20Object%20Reference) (OtherComp :type Primitive%20Component%20Object%20Reference) (OtherBodyIndex :type Integer) (bFromSweep :type Boolean) (SweepResult :type Hit%20Result%20Structure%20%28by%20ref%29))
  ;[0.15 0.15 0.15 0.5] Destroy Bait when touching sphere
  (bind _asbp_bait (Utilities|Casting|CastToBP_Bait OtherActor))
  (Actor|DestroyActor _asbp_bait))

(event EventBeginPlay
  ;[0.15 0.15 0.15 0.5] Set Himself in Game instance and give spline to boat
  (bind _returnvalue (Game|SpawnActorfromClass "/Game/ProjetUnreal2025/Blueprints/BP_Boat.BP_Boat_C" (Math|Transform|MakeTransform "0, 0, 0" "0, 0, 0" "1.000000,1.000000,1.000000") "Undefined" "MultiplyWithRoot" 0 0 0 0 0))
  (bind _asgi_fish (Utilities|Casting|CastToGI_Fish (Game|GetGameInstance)))
  (Variables|/Game/ProjetUnreal2025/Blueprints/Global/GI_Fish.GI_Fish_C|SetPlanetCenter _asgi_fish (Transformation|GetActorLocation))
  (bind _output_get (Variables|/Game/ProjetUnreal2025/Blueprints/Global/GI_Fish.GI_Fish_C|SetBoat _asgi_fish _returnvalue))
  (Variables|/Game/ProjetUnreal2025/Blueprints/BP_Boat.BP_Boat_C|SetSpline _output_get (Variables|Default|GetSpline))
  (bind _output_get_2 (Variables|Default|SetGI%20Fish _asgi_fish))
  (Variables|/Game/ProjetUnreal2025/Blueprints/Global/GI_Fish.GI_Fish_C|SetSpline _output_get_2 (Variables|Default|GetSpline))
  (Default|ChangeSelfandPawnPosition _output_get 0.0)
  (Default|SetSplinetoBoat _output_get_2))

(fn ConstructionScript)

(fn GetEdgeOfPlanetfromPoint
  (params (Point :type Vector))
  (return (* (Math|Vector|Normalize (- Point (Transformation|GetActorLocation))) (* (Transformation|GetActorScale3D) 5e+01))))