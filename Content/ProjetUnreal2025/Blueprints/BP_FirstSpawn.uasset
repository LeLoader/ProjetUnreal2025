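; BP_FirstSpawn is the initial pawn the player possesses at BeginPlay, serving as an intro camera that hands over to BP_Fisherman.
; StartMovementAnimation runs a timeline that moves it toward the fisherman's first-person camera, using a vector slerp on location.
; A timeline event starts a cubic view-target blend to the fisherman.
; On finish, it starts the boat's orbit through GI_Fish and possesses the fisherman.
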(event Custom|StartMovementAnimation
  (bind _returnvalue (Actor|GetActorOfClass "/Game/ProjetUnreal2025/Blueprints/Global/BP_Fisherman.BP_Fisherman_C"))
  (Variables|Default|SetPointEnd_Ref (Transformation|GetWorldTransform (Variables|/Game/ProjetUnreal2025/Blueprints/Global/BP_Fisherman.BP_Fisherman_C|GetFirstPersonCamera _returnvalue)))
  (Variables|Default|SetFirst%20Person%20Camera (Variables|/Game/ProjetUnreal2025/Blueprints/Global/BP_Fisherman.BP_Fisherman_C|GetFirstPersonCamera _returnvalue))
  (bind _output_get (Variables|Default|SetPointStart (Transformation|GetActorTransform)))
  (Variables|Default|SetInitialRot (.rotation _output_get))
  (Utilities|FlowControl|Sequence
    (:then_0
      (bind _track_movementcamera (Timeline|Timeline_MovementCamera PlayFromStart)
        (:Update
          (Transformation|SetActorLocation (Class|KismetMathLibrary|VectorSlerpVectortoDirection (.location (Variables|Default|GetPointStart)) (.location (Variables|Default|GetPointEnd_Ref)) _track_movementcamera) false false))
        (:Finished
          (bind _returnvalue_2 (Actor|GetActorOfClass "/Game/ProjetUnreal2025/Blueprints/Global/BP_Fisherman.BP_Fisherman_C"))
          (Default|CEStartOrbit (Variables|/Game/ProjetUnreal2025/Blueprints/Global/GI_Fish.GI_Fish_C|GetBoat (Variables|Default|GetGI%20Fish)))
          (Pawn|Possess (Game|GetPlayerController 0) _returnvalue_2))
        (:event
          (Game|Player|SetViewTargetwithBlend (Game|GetPlayerController 0) (Components|GetOwner (Variables|Default|GetFirst%20Person%20Camera)) 2.0 "VTBlend_Cubic" 0.0 false))))))

(event EventBeginPlay
  (Pawn|Possess (Game|GetPlayerController 0) self)
  (bind _asgi_fish (Utilities|Casting|CastToGI_Fish (Game|GetGameInstance)))
  (Variables|Default|SetGI%20Fish _asgi_fish))

(fn ConstructionScript)