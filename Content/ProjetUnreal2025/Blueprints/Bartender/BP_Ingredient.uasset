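; BP_Ingredient is an ingredient actor for the bartender part of the game, exposing Take and Use actions.
; Take only prints a "Took" message with the actor's display name.
; Use prints a similar message, destroys the actor and returns its DamageType value to the caller.
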(event EventTake
  (Development|PrintString (Utilities|String|Append "Took " (Utilities|GetDisplayName self))))

(fn ConstructionScript)

(fn Use
  (Development|PrintString (Utilities|String|Append "Use " (Utilities|GetDisplayName self)))
  (Actor|DestroyActor)
  (return (Variables|Default|GetDamageType)))