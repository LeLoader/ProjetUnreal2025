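; BP_BoatCPP is the boat Blueprint, driven by a lever child actor's direction changes.
; Left, right and middle call reverse, play and stop events respectively, with a motor entry or stop sound, then toggle the arms.
; The harpoon input mapping context is active only in the middle position, which is also applied on BeginPlay, so harpoon controls are unavailable while the motor runs.
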(event Custom|OnLeverDirectionChanged
  (params (NewDirection :type ELeverDirection%20Enum :default "MIDDLE") (OldDirection :type ELeverDirection%20Enum :default "MIDDLE"))
  (bind _returnvalue (Game|GetPlayerController 0))
  (bind _returnvalue_2 (PlayerController|LocalPlayerSubsystems|GetEnhancedInputLocalPlayerSubsystem _returnvalue))
  ;[0.15 0.15 0.15 0.5] CPP Version
  (switch Utilities|FlowControl|Switch|SwitchonELeverDirection NewDirection
    (:MIDDLE
      (CallFunction|CEStop)
      (Audio|PlaySound2D (Variables|Default|GetMotorStopSound) 1.0 1.0 0.0 0 0)
      (Input|AddMappingContext _returnvalue_2 "/Game/ProjetUnreal2025/Inputs/IMC_Harpoon.IMC_Harpoon" 1 "(bIgnoreAllPressedKeysUntilRelease=True,bForceImmediately=False,bNotifyUserSettings=False)"))
    (:LEFT
      (CallFunction|CEReverse)
      (Audio|PlaySound2D (Variables|Default|GetMotorEntrySound) 1.0 1.0 0.0 0 0 :!label _label)
      (Input|RemoveMappingContext _returnvalue_2 "/Game/ProjetUnreal2025/Inputs/IMC_Harpoon.IMC_Harpoon" "(bIgnoreAllPressedKeysUntilRelease=True,bForceImmediately=False,bNotifyUserSettings=False)"))
    (:RIGHT
      (CallFunction|CEPlay)
      (goto _label)))
  (Default|CallToggleArms))

(event EventBeginPlay
  (|CallParentFunction)
  (bind _asbp_lever_cpp (Utilities|Casting|CastToBP_LeverCPP (Variables|/Script/Engine.ChildActorComponent|GetChildActor (Variables|Default|GetLever))))
  (EventDispatchers|BindEventtoOnLeverDirectionChanged _asbp_lever_cpp (EventDispatchers|CreateEvent :!event OnLeverDirectionChangedSave))
  (CallFunction|OnLeverDirectionChanged "MIDDLE" "MIDDLE")
  (Input|AddMappingContext (PlayerController|LocalPlayerSubsystems|GetEnhancedInputLocalPlayerSubsystem (Game|GetPlayerController 0)) "/Game/ProjetUnreal2025/Inputs/IMC_Harpoon.IMC_Harpoon" 1 "(bIgnoreAllPressedKeysUntilRelease=True,bForceImmediately=False,bNotifyUserSettings=False)"))

(event Collision|EventActorBeginOverlap
  (params (OtherActor :type Actor%20Object%20Reference)))

(fn ConstructionScript
  (|CallParentFunction))