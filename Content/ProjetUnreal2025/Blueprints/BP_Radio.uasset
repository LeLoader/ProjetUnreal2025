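; BP_Radio is an interactable radio that plays music from BeginPlay and switches sound on interaction.
; BeginPlay spawns SoundMusic attached to the mesh, stores it as Music, and also plays the same sound in 2D.
; Interact sends a "NextSound" trigger parameter to the attached audio only.
; Show enables custom depth on the mesh for an outline, which a short timer clears.
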(event Custom|DisableOutline
  (Rendering|SetRenderCustomDepth (Variables|Default|GetMesh) false))

(event EventBeginPlay
  (bind _soundmusic (Variables|Default|GetSoundMusic))
  (bind _returnvalue (Audio|SpawnSoundAttached _soundmusic (Variables|Default|GetMesh) "None" "0, 0, 0" "0, 0, 0" "KeepRelativeOffset" false 1.0 1.0 0.0 0 0 false))
  (Variables|Default|SetMusic _returnvalue)
  (Audio|PlaySound2D _soundmusic 1.0 1.0 0.0 0 0))

(event EventShow
  (Rendering|SetRenderCustomDepth (Variables|Default|GetMesh) true)
  (Utilities|Time|SetTimerbyEvent (delegate Custom|DisableOutline) 0.05))

(event EventInteract
  (params (LeftClick :type Boolean) (IsHoldingSomething :type Boolean) (Player :type BP%20Fisherman%20Object%20Reference))
  (Class|AudioParameterControllerInterface|SetTriggerParameter(Message) (Variables|Default|GetMusic) "NextSound"))

(fn ConstructionScript)