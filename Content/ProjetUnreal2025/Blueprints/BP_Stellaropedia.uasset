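; BP_Stellaropedia is an interactable object that opens and closes an encyclopedia UI.
; It creates the UI_Encyclopedie widget on BeginPlay, and Interact alternates through a FlipFlop between adding and removing it from the viewport, each with a sound.
; Show enables custom depth on the mesh and sets a short timer to clear it, so the outline is momentary unless Show is called again.
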(event Custom|DisableOutline
  (Rendering|SetRenderCustomDepth (Variables|Default|GetMesh) false))

(event EventShow
  (Rendering|SetRenderCustomDepth (Variables|Default|GetMesh) true)
  (Utilities|Time|SetTimerbyEvent (delegate Custom|DisableOutline) 0.05))

(event EventInteract
  (params (LeftClick :type Boolean) (IsHoldingSomething :type Boolean) (Player :type BP%20Fisherman%20Object%20Reference))
  (Utilities|FlowControl|FlipFlop
    (:A
      (Audio|PlaySound2D (Variables|Default|GetOpenSound) 1.0 1.0 0.0 0 0)
      (UserInterface|Viewport|AddtoViewport (Variables|Default|GetEncyclopedia) 0))
    (:B
      (Audio|PlaySound2D (Variables|Default|GetCloseSound) 1.0 1.0 0.0 0 0)
      (Widget|RemovefromParent (Variables|Default|GetEncyclopedia)))))

(event EventBeginPlay
  (bind _returnvalue (UserInterface|CreateWidget "/Game/ProjetUnreal2025/Widgets/UI_Encyclopedie/UI_Encyclopedie.UI_Encyclopedie_C" (Game|GetPlayerController 0)))
  (Variables|Default|SetEncyclopedia _returnvalue))

(fn ConstructionScript)