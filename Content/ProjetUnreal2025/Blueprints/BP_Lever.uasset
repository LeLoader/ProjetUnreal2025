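; Interactable three-position lever that steps a movement direction between Forward, Stopped and Backward on left or right click.
; Each step plays a sound, sets a target rotation that Tick eases toward, and broadcasts the new direction through CallLeft or CallRight.
; Interacting while holding something also sends the held object a reeled message.
; Show briefly outlines the meshes via custom depth and a timer; a separate timeline rotation event has no caller here.
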(event Custom|DisableOutline
  (Rendering|SetRenderCustomDepth (Variables|Default|GetSM_Lever) false)
  (Rendering|SetRenderCustomDepth (Variables|Default|GetSM_LeverBase) false))

(event Custom|CE_StartRotation
  (params (negative :type Float%20%28double-precision%29) (XAtStart :type Float%20%28double-precision%29))
  (bind _float (Timeline|Timeline PlayFromStart)
    (:Update
      (Transformation|SetRelativeRotation (Variables|Default|GetSM_Lever) (Math|Rotator|MakeRotator (Math|Float|Lerp XAtStart (+ (* negative 4e+01) XAtStart) _float) 0.0 0.0) false false))))

(event EventTick
  (params (DeltaSeconds :type Float%20%28single-precision%29))
  (bind _sm_lever (Variables|Default|GetSM_Lever))
  (Transformation|SetRelativeRotation _sm_lever (Math|Interpolation|RInterpTo (Variables|/Script/Engine.SceneComponent|GetRelativeRotation _sm_lever) (Variables|Default|GetTargetRotation) DeltaSeconds 1e+01) false false))

(event EventShow
  (Rendering|SetRenderCustomDepth (Variables|Default|GetSM_Lever) true)
  (Rendering|SetRenderCustomDepth (Variables|Default|GetSM_LeverBase) true)
  (Utilities|Time|SetTimerbyEvent (delegate Custom|DisableOutline) 0.05))

(event EventInteract
  (params (LeftClick :type Boolean) (IsHoldingSomething :type Boolean) (Player :type BP%20Fisherman%20Object%20Reference))
  (if IsHoldingSomething
    (Class|BPIHarpoonable|OnReeled(Message) (Variables|/Game/ProjetUnreal2025/Blueprints/Global/BP_Fisherman.BP_Fisherman_C|GetHeldObject Player) Player))
  (if LeftClick
    (Development|PrintString "clicked Left")
    (switch Utilities|FlowControl|Switch|SwitchonE_Movement (Variables|Default|GetMovementDirection)
      (:NewEnumerator0
        (Variables|Default|SetMovementDirection "NewEnumerator1")
        (Audio|PlaySound2D (Variables|Default|GetStopSound) 1.0 1.0 0.0 0 0)
        (Variables|Default|SetTargetRotation (Variables|Default|GetCenterRotation)))
      (:NewEnumerator1
        (Variables|Default|SetMovementDirection "NewEnumerator2")
        (Audio|PlaySound2D (Variables|Default|GetInteractSound) 1.0 1.0 0.0 0 0)
        (Variables|Default|SetTargetRotation (Variables|Default|GetLeftRotation))))
    (Default|CallCallLeft (Variables|Default|GetMovementDirection))
    (else
      (Development|PrintString "clicked right")
      (switch Utilities|FlowControl|Switch|SwitchonE_Movement (Variables|Default|GetMovementDirection)
        (:NewEnumerator1
          (Variables|Default|SetMovementDirection "NewEnumerator0")
          (Audio|PlaySound2D (Variables|Default|GetInteractSound) 1.0 1.0 0.0 0 0)
          (Variables|Default|SetTargetRotation (Variables|Default|GetRightRotation)))
        (:NewEnumerator2
          (Variables|Default|SetMovementDirection "NewEnumerator1")
          (Audio|PlaySound2D (Variables|Default|GetStopSound) 1.0 1.0 0.0 0 0)
          (Variables|Default|SetTargetRotation (Variables|Default|GetCenterRotation))))
      (Default|CallCallRight (Variables|Default|GetMovementDirection)))))

(event EventBeginPlay
  (Variables|Default|SetMovementDirection "NewEnumerator1")
  (Components|Timeline|SetPlayRate (Variables|Default|GetTimeline) 5.0)
  (Variables|Default|SetTargetRotation (Variables|Default|GetCenterRotation)))

(fn ConstructionScript)