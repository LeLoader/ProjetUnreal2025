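; BP_Empty_Bernard is an actor that keeps turning to face the BP_Boat actor in the level.
; On Tick it rotates toward the cached boat using a look-at rotation, or finds the boat by class when that reference is invalid.
; A ClearBernardInside event, taking a destroyed actor, resets the BernardInside flag to false.
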(event Custom|ClearBernardInside
  (params (Destroyed%20Actor :type Actor%20Object%20Reference))
  (Variables|Default|SetBernardInside false))

(event EventBeginPlay)

(event Collision|EventActorBeginOverlap
  (params (OtherActor :type Actor%20Object%20Reference)))

(event EventTick
  (params (DeltaSeconds :type Float%20%28single-precision%29))
  (Utilities|IsValid (Variables|Default|GetBoat)
    (:Is%20Valid
      (Transformation|SetActorRotation (Math|Rotator|FindLookatRotation (Transformation|GetActorLocation) (Transformation|GetActorLocation (Variables|Default|GetBoat)))))
    (:Is%20Not%20Valid
      (bind _returnvalue (Actor|GetActorOfClass "/Game/ProjetUnreal2025/Blueprints/BP_Boat.BP_Boat_C"))
      (Variables|Default|SetBoat _returnvalue))))

(fn ConstructionScript)