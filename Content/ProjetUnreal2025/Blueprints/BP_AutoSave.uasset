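; BP_AutoSave is an auto-save actor that writes the boat's bait counts to a save game.
; BeginPlay caches the GI_Fish game instance as the data source.
; Every Tick, and on CE_Debug, it constructs a new SG_SaveSystem, copies the Somalite, Glugmalite and Methacite bait numbers into it, and saves synchronously.
; The slot name is empty, and a printed message reports success or failure.
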(event Custom|CE_Debug
  (bind _gi_fish (Variables|Default|GetGI%20Fish))
  (bind _boat (Variables|/Game/ProjetUnreal2025/Blueprints/Global/GI_Fish.GI_Fish_C|GetBoat _gi_fish))
  (bind _returnvalue (Game|ConstructObjectfromClass "/Game/ProjetUnreal2025/Blueprints/Global/SG_SaveSystem.SG_SaveSystem_C"))
  (Utilities|Struct|SetmembersinS_SaveBaitNumber (Variables|/Game/ProjetUnreal2025/Blueprints/Global/SG_SaveSystem.SG_SaveSystem_C|GetBaitNumber _returnvalue) (Variables|/Game/ProjetUnreal2025/Blueprints/BP_Boat.BP_Boat_C|GetSomaliteBaitNumber _boat) (Variables|/Game/ProjetUnreal2025/Blueprints/BP_Boat.BP_Boat_C|GetGlugmaliteBaitNumber _boat) (Variables|/Game/ProjetUnreal2025/Blueprints/BP_Boat.BP_Boat_C|GetMethaciteBaitNumber _boat))
  (bind _returnvalue_2 (SaveGame|SaveGametoSlot _returnvalue))
  (if _returnvalue_2
    (Development|PrintString "Auto Save Successful")
    (else
      (Development|PrintString "Auto Save Failed"))))

(event EventBeginPlay
  (bind _asgi_fish (Utilities|Casting|CastToGI_Fish (Game|GetGameInstance)))
  (Variables|Default|SetGI%20Fish _asgi_fish))

(event EventTick
  (params (DeltaSeconds :type Float%20%28single-precision%29))
  (bind _gi_fish (Variables|Default|GetGI%20Fish))
  (bind _boat (Variables|/Game/ProjetUnreal2025/Blueprints/Global/GI_Fish.GI_Fish_C|GetBoat _gi_fish))
  (bind _returnvalue (Game|ConstructObjectfromClass "/Game/ProjetUnreal2025/Blueprints/Global/SG_SaveSystem.SG_SaveSystem_C"))
  (Utilities|Struct|SetmembersinS_SaveBaitNumber (Variables|/Game/ProjetUnreal2025/Blueprints/Global/SG_SaveSystem.SG_SaveSystem_C|GetBaitNumber _returnvalue) (Variables|/Game/ProjetUnreal2025/Blueprints/BP_Boat.BP_Boat_C|GetSomaliteBaitNumber _boat) (Variables|/Game/ProjetUnreal2025/Blueprints/BP_Boat.BP_Boat_C|GetGlugmaliteBaitNumber _boat) (Variables|/Game/ProjetUnreal2025/Blueprints/BP_Boat.BP_Boat_C|GetMethaciteBaitNumber _boat))
  (bind _returnvalue_2 (SaveGame|SaveGametoSlot _returnvalue))
  (if _returnvalue_2
    (Development|PrintString "Auto Save Successful")
    (else
      (Development|PrintString "Auto Save Failed"))))

(fn ConstructionScript)