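; BP_Bait is a throwable bait actor that the fisherman can launch, harpoon and reel back in.
; Throwing clears the player's held object, starts a movement component along the camera's forward vector and sets a 60-second self-destruct timer.
; On reel-in it tries to store itself in the boat's bait box via the game instance, destroying itself on success or getting thrown again otherwise.
; Events slow, stop (when eaten) or shrink-and-destroy it.
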(event Custom|CE_ThrowBait
  (bind _throwmovement (Variables|Default|GetThrowMovement))
  (Utilities|Time|SetTimerbyEvent (delegate Custom|CE_Destroy) 6e+01)
  (bind _asbp_fisherman (Utilities|Casting|CastToBP_Fisherman (Game|Player|GetPlayerPawn 0)))
  (Variables|/Game/ProjetUnreal2025/Blueprints/Global/BP_Fisherman.BP_Fisherman_C|SetHeldObject _asbp_fisherman 0)
  (Variables|/Script/Engine.MovementComponent|SetVelocity _throwmovement (* (Math|Vector|GetForwardVector (Variables|/Script/Engine.PlayerCameraManager|GetTransformComponent (Game|GetPlayerCameraManager 0))) (Variables|Default|GetThrowStrength)))
  (Components|Activation|Activate _throwmovement false))

(event Custom|CE_ReduceSpeed
  (bind _throwmovement (Variables|Default|GetThrowMovement))
  (Variables|/Script/Engine.MovementComponent|SetVelocity _throwmovement (* (Variables|/Script/Engine.MovementComponent|GetVelocity _throwmovement) (Math|Float|Min(Float) (/ 1.0 (Variables|Default|GetReducingAmount)) 1.0))))

(event Custom|CE_Destroy
  (Development|PrintString "committing suicide")
  (Actor|DestroyActor))

(event Custom|Eat
  (Components|Activation|Deactivate (Variables|Default|GetThrowMovement))
  (Development|PrintString "Eaten"))

(event Custom|CE_Shrink
  (Variables|Default|SetStartScale (Transformation|GetActorScale3D))
  (bind _float (Timeline|Timeline PlayFromStart)
    (:Update
      (Transformation|SetActorScale3D (Math|Vector|Lerp(Vector) (Variables|Default|GetStartScale) "0, 0, 0" _float)))
    (:Finished
      (Actor|DestroyActor))))

(event EventBeginPlay
  (Components|Activation|Deactivate (Variables|Default|GetThrowMovement))
  (Development|PrintString "Spawned")
  (bind _asgi_fish (Utilities|Casting|CastToGI_Fish (Game|GetGameInstance))
    (:then
      (Variables|Default|SetGI%20Fish _asgi_fish))
    (:CastFailed
      (Development|PrintString "Uh"))))

(event EventDestroyed
  (Development|PrintString "Bait got destroyed"))

(event EventTick
  (params (DeltaSeconds :type Float%20%28single-precision%29))
  ;[0.15 0.15 0.15 0.5] Code For Gravitating, needs to inherit bp gravity and put gravity Movement instead of throw
)

(event EventOnReeled
  ;[0.15 0.15 0.15 0.5] got retrieved by the player, trying to put in a box
  (Development|PrintString "reeled")
  (bind _didput (Default|PutBaitinBox (Variables|/Game/ProjetUnreal2025/Blueprints/Global/GI_Fish.GI_Fish_C|GetBoat (Variables|Default|GetGI%20Fish)) (Variables|Default|GetBaitType)))
  (if _didput
    (Actor|DestroyActor)
    (else
      (CallFunction|CEThrowBait))))

(fn ConstructionScript)

(fn CanbeReeled
  (return true))

(fn OnHarpooned
  (Audio|PlaySound2D (Variables|Default|GetBaitSound) 1.0 1.0 0.0 0 0)
  (Default|CallHarpooned self)
  (bind _canbereeled (CallFunction|CanbeReeled))
  (return _canbereeled false))