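; BP_FakeBait is a projectile bait actor that advertises itself through AI noise events, apparently to attract fish.
; On BeginPlay it sets its velocity along the gravity vector that BP_FishNavBounds returns for its location, scaled by BaitSpeed, and randomly picks one of two bait types.
; Each tick it reports noise at its location, tagged with the bait type name, as long as its Sensed flag is false.
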(event EventBeginPlay
  (bind _returnvalue (Actor|GetActorOfClass "/Game/ProjetUnreal2025/Blueprints/Actors/Fish/BP_FishNavBounds.BP_FishNavBounds_C"))
  (Variables|/Script/Engine.MovementComponent|SetVelocity (Variables|Default|GetProjectileMovement) (* (Default|GetGravityVector _returnvalue (Transformation|GetActorLocation)) (Variables|Default|GetBaitSpeed)))
  (Variables|Default|SetBaitType (select (Math|Random|RandomBool) "NewEnumerator1" "NewEnumerator0")))

(event EventTick
  (params (DeltaSeconds :type Float%20%28single-precision%29))
  (if (not (Variables|Default|GetSensed))
    (Class|AISenseHearing|ReportNoiseEvent (Transformation|GetActorLocation) 1.0 self 0.0 (Utilities|Name|EnumtoName (Variables|Default|GetBaitType)))))

(fn ConstructionScript)