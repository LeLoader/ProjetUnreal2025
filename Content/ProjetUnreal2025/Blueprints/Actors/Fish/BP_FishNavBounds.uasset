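; BP_FishNavBounds defines a spherical shell between inner and outer spheres as fish bounds and spawns one BP_FishPawn there on BeginPlay.
; The construction script sizes both spheres; random points are origin-relative, using recursive retries to exclude directions near the poles.
; A random DT_Fishs row only feeds a debug print, which re-rolls the reported location.
; Path-to-point and sphere-intersection functions are unfinished stubs.
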(event EventBeginPlay
  (CallFunction|SpawnRandomFish))

(fn ConstructionScript
  (Components|Sphere|SetSphereRadius (Variables|Default|GetInnerSphere) (Variables|Default|GetInnerSphereRadius) false)
  (Components|Sphere|SetSphereRadius (Variables|Default|GetExtSphere) (Variables|Default|GetExtSphereRadius) false))

(fn GetRandomPointinBounds
  (params (ZBoundsPercentage :type Float%20%28double-precision%29))
  (bind _returnvalue (* ZBoundsPercentage 2.0))
  (LocalVariables|SetRandomUnitVector (Math|Random|RandomUnitVector))
  (if (Math|Float|InRange(Float) (.Z (Math|Vector|BreakVector (LocalVariables|GetRandomUnitVector))) (+ _returnvalue -1.0) (- 1.0 _returnvalue))
    (return (* (Math|Random|RandomFloatinRange (Variables|Default|GetInnerSphereRadius) (Variables|Default|GetExtSphereRadius)) (Math|Vector|MakeVector (.X (Math|Vector|BreakVector (LocalVariables|GetRandomUnitVector))) (.Y (Math|Vector|BreakVector (LocalVariables|GetRandomUnitVector))) (.Z (Math|Vector|BreakVector (LocalVariables|GetRandomUnitVector))))))
    (else
      (return (CallFunction|GetRandomPointinBounds ZBoundsPercentage)))))

(fn SpawnRandomFish
  (bind _position (CallFunction|GetRandomPointinBounds 0.2))
  (bind _outrownames (DataTable|GetDataTableRowNames "/Game/ProjetUnreal2025/Data/DT_Fishs.DT_Fishs"))
  (bind _returnvalue (Utilities|GetDataTableRow "/Game/ProjetUnreal2025/Data/DT_Fishs.DT_Fishs" (.OutItem (Utilities|Array|Random _outrownames)))
    (:then
      (Game|SpawnActorfromClass "/Game/ProjetUnreal2025/Blueprints/Actors/Fish/BP_FishPawn.BP_FishPawn_C" (Math|Transform|MakeTransform _position "0, 0, 0" "1.000000,1.000000,1.000000") "AlwaysSpawn" "MultiplyWithRoot" 0 0)
      (Development|PrintText (Utilities|Text|FormatText (Class|KismetTextLibrary|MakeInvariantText "Spawned a fish ({0}) at {1}, with favorite bait {2}") (.Name (Utilities|Struct|BreakS_Fish _returnvalue)) (Utilities|String|ToString(Vector) _position) (Utilities|Name|EnumtoName (.Bait (Utilities|Struct|BreakS_Fish _returnvalue)))) true true "(R=0.000000,G=0.660000,B=1.000000,A=1.000000)" 2e+01))))

(fn GetPathtoPoint
  (params (StartPosition :type Vector) (EndPosition :type Vector)))

(fn DoesVectorIntersectwithSphere
  (params (SpherePosition :type Vector) (SphereRadius :type Float%20%28double-precision%29) (PointPosition :type Vector) (Direction :type Vector))
  (return false))