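; BP_Lever is an interactable three-position lever that sets a movement direction of Forward, Stopped or Backward, starting at Forward on BeginPlay.
; Interact shifts it one position toward Backward on left click or toward Forward otherwise, ignoring input past either end.
; Each shift rolls the lever mesh by a fixed step and broadcasts the new direction through the CallLeft or CallRight dispatcher.
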(event EventInteract
  (params (LeftClick :type Boolean))
  (bind _sm_lever (Variables|Default|GetSM_Lever))
  (if LeftClick
    (Development|PrintString "clicked Left")
    (switch Utilities|FlowControl|Switch|SwitchonE_Movement (Variables|Default|GetMovementDirection)
      (:NewEnumerator0
        (Variables|Default|SetMovementDirection "NewEnumerator1"))
      (:NewEnumerator1
        (Variables|Default|SetMovementDirection "NewEnumerator2")))
    (Transformation|AddRelativeRotation _sm_lever (Math|Rotator|MakeRotator -4e+01 0.0 0.0) false false)
    (Default|CallCallLeft (Variables|Default|GetMovementDirection))
    (else
      (Development|PrintString "clicked right")
      (switch Utilities|FlowControl|Switch|SwitchonE_Movement (Variables|Default|GetMovementDirection)
        (:NewEnumerator1
          (Variables|Default|SetMovementDirection "NewEnumerator0"))
        (:NewEnumerator2
          (Variables|Default|SetMovementDirection "NewEnumerator1")))
      (Transformation|AddRelativeRotation _sm_lever (Math|Rotator|MakeRotator 4e+01 0.0 0.0) false false)
      (Default|CallCallRight (Variables|Default|GetMovementDirection)))))

(event EventBeginPlay
  (Variables|Default|SetMovementDirection "NewEnumerator0"))

(fn ConstructionScript)