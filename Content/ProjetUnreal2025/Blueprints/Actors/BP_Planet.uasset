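; BP_Planet is a planet actor that carries the player pawn along a spline path and can spawn fish on its sphere.
; A slowed, restarting timeline moves the pawn along the spline, adding the look-at rotation toward the sphere to its rotation on each update.
; CE_SpawnFish places a BP_Fish2 at a random point on the scaled sphere, facing outward from the center.
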(event Custom|CE_Restart
  (bind _returnvalue (Game|Player|GetPlayerPawn 0))
  (bind _spline (Variables|Default|GetSpline))
  (bind _track (Timeline|Timeline PlayFromStart)
    (:Update
      (Transformation|SetActorLocation _returnvalue (.location (Spline|GetTransformatDistanceAlongSpline _spline (Math|Float|Lerp 0.0 (Spline|GetSplineLength _spline) _track) "World" false)) false false)
      (Class|Actor|AddActorWorldRotation _returnvalue (Math|Rotator|FindLookatRotation (Transformation|GetActorLocation _returnvalue) (Transformation|GetWorldLocation (Variables|Default|GetSphere)))))
    (:Finished
      (CallFunction|CERestart))))

(event Custom|CE_SpawnFish
  (bind _returnvalue (Math|Random|RandomUnitVector))
  (bind _sphere (Variables|Default|GetSphere))
  (bind _returnvalue_2 (Transformation|GetWorldLocation _sphere))
  (bind _returnvalue_3 (Transformation|GetWorldScale _sphere))
  (bind _returnvalue_4 (* _returnvalue _returnvalue_3))
  (bind _returnvalue_5 (* _returnvalue_4 5e+01))
  (bind _returnvalue_6 (+ _returnvalue_5 _returnvalue_2))
  (Game|SpawnActorfromClass "/Game/ProjetUnreal2025/Blueprints/Actors/BP_Fish2.BP_Fish2_C" (Math|Transform|MakeTransform _returnvalue_6 (Math|Rotator|FindLookatRotation (Transformation|GetWorldLocation (Variables|Default|GetSphere)) _returnvalue_6) "1.000000,1.000000,1.000000") "Undefined" "MultiplyWithRoot" 0 0))

(event EventBeginPlay
  (bind _returnvalue (Game|Player|GetPlayerPawn 0))
  (bind _spline (Variables|Default|GetSpline))
  (Components|Timeline|SetPlayRate (Variables|Default|GetTimeline) 0.01)
  (bind _track (Timeline|Timeline PlayFromStart)
    (:Update
      (Transformation|SetActorLocation _returnvalue (.location (Spline|GetTransformatDistanceAlongSpline _spline (Math|Float|Lerp 0.0 (Spline|GetSplineLength _spline) _track) "World" false)) false false)
      (Class|Actor|AddActorWorldRotation _returnvalue (Math|Rotator|FindLookatRotation (Transformation|GetActorLocation _returnvalue) (Transformation|GetWorldLocation (Variables|Default|GetSphere)))))
    (:Finished
      (CallFunction|CERestart))))

(fn ConstructionScript)