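; BP_Bait is a bait actor that can jump toward the planet referenced by the GI_Fish game instance.
; CE_GoTowardsPlanet reads that planet's location and instantly sets the bait's position a fixed fraction of the way there through a vector lerp, without sweeping.
; Debug prints report the call, the target position and a failed game instance cast.
; BeginPlay is empty and a Timeline node is left unconnected.
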(event Custom|CE_GoTowardsPlanet
  (Development|PrintString "Spawned")
  (bind _asgi_fish (Utilities|Casting|CastToGI_Fish (Game|GetGameInstance))
    (:then
      (Development|PrintString (Utilities|String|ToString(Vector) (Math|Vector|Lerp(Vector) (Transformation|GetActorLocation) (Transformation|GetActorLocation (Variables|/Game/ProjetUnreal2025/Blueprints/GI_Fish.GI_Fish_C|GetPlanet _asgi_fish)) 0.6)))
      (Transformation|SetActorLocation (Math|Vector|Lerp(Vector) (Transformation|GetActorLocation) (Transformation|GetActorLocation (Variables|/Game/ProjetUnreal2025/Blueprints/GI_Fish.GI_Fish_C|GetPlanet _asgi_fish)) 0.6) false false))
    (:CastFailed
      (Development|PrintString "Uh"))))

(event EventBeginPlay)

(fn ConstructionScript)