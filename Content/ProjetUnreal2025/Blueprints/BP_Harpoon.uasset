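; Harpoon projectile that detaches, shows its cable and flies along the control rotation when fired, reporting what it hooks.
; On firing, a camera sphere trace enables homing on the first reelable target found.
; Hitting a willing BPI_Harpoonable actor attaches it to the harpoon and broadcasts it with a manual-reel flag.
; Other hits, overlaps or a free-flight timeout broadcast without an object; hits and overlaps also stop movement.
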(event OnComponentHit(Harpoon)
  (params (HitComponent :type Primitive%20Component%20Object%20Reference) (OtherActor :type Actor%20Object%20Reference) (OtherComp :type Primitive%20Component%20Object%20Reference) (NormalImpulse :type Vector :default "0, 0, 0") (Hit :type Hit%20Result%20Structure%20%28by%20ref%29))
  ;[0.15 0.15 0.15 0.5] On HarpoonComponent Hit
  (if (Utilities|DoesObjectImplementInterface OtherActor "/Game/ProjetUnreal2025/Interfaces/BPI_Harpoonable.BPI_Harpoonable_C")
    (bind (_success _manualreel) (Class|BPIHarpoonable|OnHarpooned(Message) OtherActor))
    (if _success
      (Default|CallOnHarpoonSomething OtherActor _manualreel)
      (Variables|Default|SetHookedObject OtherActor)
      (Transformation|SetWorldLocation (Variables|Default|GetHarpoon) (.ImpactPoint (Collision|BreakHitResult Hit)) false false)
      (Transformation|AttachActorToActor OtherActor self "None" "KeepWorld" "KeepWorld" "KeepWorld" true)
      (CallFunction|StopMovement)
      (else
        (Default|CallOnHarpoonSomething 0 false :!label _label)
        (CallFunction|StopMovement)))
    (else
      (goto _label))))

(event OnComponentBeginOverlap(Harpoon)
  (params (OverlappedComponent :type Primitive%20Component%20Object%20Reference) (OtherActor :type Actor%20Object%20Reference) (OtherComp :type Primitive%20Component%20Object%20Reference) (OtherBodyIndex :type Integer) (bFromSweep :type Boolean) (SweepResult :type Hit%20Result%20Structure%20%28by%20ref%29))
  ;[0.15 0.15 0.15 0.5] On HarpoonComponent Hit
  (Default|CallOnHarpoonSomething 0 false)
  (CallFunction|StopMovement))

(event Custom|StopMovement
  (bind _projectilemovement (Variables|Default|GetProjectileMovement))
  (Components|Movement|StopMovementImmediately _projectilemovement)
  (Components|Activation|Deactivate _projectilemovement)
  (Variables|/Script/Engine.ProjectileMovementComponent|SetbIsHomingProjectile _projectilemovement false)
  (Variables|/Script/Engine.ProjectileMovementComponent|SetHomingTargetComponent _projectilemovement 0)
  (Utilities|Time|ClearandInvalidateTimerbyHandle (Variables|Default|GetTimer)))

(event Custom|OnMaxFreeTimeReached
  (Default|CallOnHarpoonSomething 0 false))

(event EventBeginPlay
  (Rendering|SetVisibility (Variables|Default|GetCable) false false))

(fn ConstructionScript)

(fn Fire
  (params (ControlRotation :type Rotator))
  (bind _projectilemovement (Variables|Default|GetProjectileMovement))
  (bind _projectilemovement_2 (Variables|Default|GetProjectileMovement))
  (Variables|/Script/Engine.ProjectileMovementComponent|SetHomingTargetComponent _projectilemovement_2 0)
  (Variables|/Script/Engine.ProjectileMovementComponent|SetbIsHomingProjectile _projectilemovement_2 false)
  (if (not (Variables|Default|GetIsFired))
    (CallFunction|CheckforObject)
    (Variables|/Script/Engine.MovementComponent|SetVelocity _projectilemovement (* (* (Variables|Default|GetFireSpeed) 1e+02) (Math|Vector|GetForwardVector ControlRotation)))
    (Components|Activation|Activate _projectilemovement false)
    (Rendering|SetVisibility (Variables|Default|GetCable) true false)
    (Transformation|DetachFromActor "KeepWorld" "KeepWorld" "KeepWorld")
    (Audio|PlaySound2D (Variables|Default|GetFireSound) 1.0 1.0 0.0 0 0)
    (bind _returnvalue (Utilities|Time|SetTimerbyEvent (EventDispatchers|CreateEvent :!event Custom|OnMaxFreeTimeReached) (Variables|Default|GetMaxFreeTime)))
    (Variables|Default|SetTimer _returnvalue)
    (bind _output_get (Variables|Default|SetIsFired true))
    (return _output_get)
    (else
      (return false))))

(fn CheckforObject
  (bind _returnvalue (Game|GetPlayerCameraManager 0))
  (bind _projectilemovement (Variables|Default|GetProjectileMovement))
  (bind _returnvalue_2 (Camera|GetCameraLocation _returnvalue))
  (bind (_outhits _returnvalue_3) (Collision|MultiSphereTraceForObjects _returnvalue_2 (+ _returnvalue_2 (* (Math|Vector|GetForwardVector (Variables|/Script/Engine.PlayerCameraManager|GetTransformComponent _returnvalue)) 2e+03)) (Variables|Default|GetHomingRange) (Utilities|Array|MakeArray "ObjectTypeQuery9" "ObjectTypeQuery10") false 0 "ForOneFrame"))
  (if _returnvalue_3
    (bind _array_element (Utilities|Array|ForEachLoopwithBreak _outhits :!label _label)
      (:LoopBody
        (bind _canbereeled (Class|BPIHarpoonable|CanbeReeled(Message) (.HitActor (Collision|BreakHitResult _array_element))))
        (if _canbereeled
          (Variables|/Script/Engine.ProjectileMovementComponent|SetbIsHomingProjectile _projectilemovement true)
          (Variables|/Script/Engine.ProjectileMovementComponent|SetHomingTargetComponent _projectilemovement (.HitComponent (Collision|BreakHitResult _array_element)))
          (goto _label Break))))))