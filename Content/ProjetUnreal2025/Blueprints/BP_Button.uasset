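; Interactable big button under a glass cover that ends the game or level by showing the WBP_End screen.
; CE_Open makes it interactable and sets a target rotation, which Tick smoothly interpolates the glass cover toward.
; Show briefly outlines the button through custom depth on a short timer, only while it is interactable.
; Interact creates the end widget, then, if unlocked, fires Leave and adds the widget to the viewport.
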(event Custom|DisableOutline
  (Rendering|SetRenderCustomDepth (Variables|Default|GetMode_Bigboutton_bouton) false))

(event Custom|CE_Open
  (Variables|Default|SetCanBeInteracted true)
  (Variables|Default|SetTargetRotation "0.000000,0.000000,-90.000000"))

(event EventInteract
  (params (LeftClick :type Boolean) (IsHoldingSomething :type Boolean) (Player :type BP%20Fisherman%20Object%20Reference))
  (bind _returnvalue (UserInterface|CreateWidget "/Game/ProjetUnreal2025/Widgets/WBP_End.WBP_End_C"))
  (if (Variables|Default|GetCanBeInteracted)
    (Default|CallLeave)
    (UserInterface|Viewport|AddtoViewport _returnvalue 0)))

(event EventShow
  (if (Variables|Default|GetCanBeInteracted)
    (Rendering|SetRenderCustomDepth (Variables|Default|GetMode_Bigboutton_bouton) true)
    (Utilities|Time|SetTimerbyEvent (delegate Custom|DisableOutline) 0.05)))

(event EventTick
  (params (DeltaSeconds :type Float%20%28single-precision%29))
  (bind _mode_bigboutton_verre (Variables|Default|GetMode_Bigboutton_verre))
  (Transformation|SetRelativeRotation _mode_bigboutton_verre (Math|Interpolation|RInterpTo (Variables|/Script/Engine.SceneComponent|GetRelativeRotation _mode_bigboutton_verre) (Variables|Default|GetTargetRotation) DeltaSeconds 3.0) false false))

(fn ConstructionScript)