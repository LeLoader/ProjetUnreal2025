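; AI-controlled fish pawn that senses and eats bait, jumps under planet gravity, and can be harpooned and reeled in.
; The detection zone writes one bait to the Blackboard, pausing until it is destroyed; the eating zone destroys overlapped bait.
; Jumping enables physics, harpooning and a radial pull toward world origin until Root overlaps or a harpoon hits.
; Harpooning sets IsHooked; dropping clears it and restarts the jump, while reeling destroys the fish.
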(event OnComponentBeginOverlap(FishEatingZone)
  (params (OverlappedComponent :type Primitive%20Component%20Object%20Reference) (OtherActor :type Actor%20Object%20Reference) (OtherComp :type Primitive%20Component%20Object%20Reference) (OtherBodyIndex :type Integer) (bFromSweep :type Boolean) (SweepResult :type Hit%20Result%20Structure%20%28by%20ref%29))
  (Variables|Default|SetBait OtherActor)
  (Utilities|Time|SetTimerbyEvent (delegate Custom|EatBait) 0.01)
  (Default|CallOnGetBait))

(event OnComponentBeginOverlap(FishDetectionZone)
  (params (OverlappedComponent :type Primitive%20Component%20Object%20Reference) (OtherActor :type Actor%20Object%20Reference) (OtherComp :type Primitive%20Component%20Object%20Reference) (OtherBodyIndex :type Integer) (bFromSweep :type Boolean) (SweepResult :type Hit%20Result%20Structure%20%28by%20ref%29))
  (Game|BindEventtoOnDestroyed OtherActor (delegate Custom|ClearTargetBait))
  (AI|Components|Blackboard|SetValueasObject (Variables|/Script/AIModule.AIController|GetBlackboard (AI|GetAIController self)) (Utilities|Name|MakeLiteralName "SensedBait") OtherActor)
  (Collision|SetCollisionEnabled (Variables|Default|GetFishDetectionZone) "NoCollision"))

(event OnComponentBeginOverlap(Root)
  (params (OverlappedComponent :type Primitive%20Component%20Object%20Reference) (OtherActor :type Actor%20Object%20Reference) (OtherComp :type Primitive%20Component%20Object%20Reference) (OtherBodyIndex :type Integer) (bFromSweep :type Boolean) (SweepResult :type Hit%20Result%20Structure%20%28by%20ref%29))
  (Default|CallOnHitPlanet)
  (CallFunction|EndJump))

(event Custom|Jump
  (Physics|SetSimulatePhysics (Variables|Default|GetRoot) true)
  (Variables|Default|SetIsGravityEnabled true)
  (Variables|Default|SetHarpoonable true))

(event Custom|EndJump
  (Physics|SetSimulatePhysics (Variables|Default|GetRoot) false)
  (Variables|Default|SetIsGravityEnabled false)
  (Variables|Default|SetHarpoonable false))

(event Custom|ClearTargetBait
  (params (DestroyedActor :type Actor%20Object%20Reference))
  ;[0.15 0.15 0.15 0.5] Eaten or destroyed by planet
  (Game|UnbindEventfromOnDestroyed DestroyedActor (delegate Custom|ClearTargetBait))
  (AI|Components|Blackboard|ClearValue (Variables|/Script/AIModule.AIController|GetBlackboard (AI|GetAIController self)) (Utilities|Name|MakeLiteralName "SensedBait"))
  (Class|KismetSystemLibrary|SetTimerforNextTickDelegate (delegate Custom|Reactivate%20Collision))
  (Default|CallOnTargetBaitGotDestroyed))

(event Custom|Reactivate%20Collision
  (Collision|SetCollisionEnabled (Variables|Default|GetFishDetectionZone) "QueryAndPhysics"))

(event Custom|EatBait
  (Actor|DestroyActor (Variables|Default|GetBait)))

(event EventTick
  (params (DeltaSeconds :type Float%20%28single-precision%29))
  (if (Variables|Default|GetIsGravityEnabled)
    (Physics|AddRadialForce (Variables|Default|GetRoot) "0, 0, 0" 1e+05 (* (Variables|Default|GetGravityStrenght) -1e+02) "RIF_Constant" true)))

(event EventOnDrop
  (Transformation|DetachFromActor "KeepWorld" "KeepWorld" "KeepWorld")
  (AI|Components|Blackboard|SetValueasBool (AI|GetBlackboard (AI|GetAIController self)) (Utilities|Name|MakeLiteralName "IsHooked") false)
  (CallFunction|Jump))

(event EventOnReeled
  (Default|CallGotReeled)
  (Actor|DestroyActor))

(fn ConstructionScript)

(fn OnHarpooned
  (if (Variables|Default|GetHarpoonable)
    (AI|Components|Blackboard|SetValueasBool (AI|GetBlackboard (AI|GetAIController self)) (Utilities|Name|MakeLiteralName "IsHooked") true)
    (CallFunction|EndJump)
    (return true true)
    (else
      (return false false))))