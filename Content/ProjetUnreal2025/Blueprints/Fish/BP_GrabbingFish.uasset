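; Grabbing fish variant that takes the bait and escapes to a safe zone unless it is harpooned enough times.
; Catching bait starts a timer that, on expiry, signals the safe zone was reached and resets the hit count.
; Each harpoon adds a hit, and the parent harpoon logic runs only once the reelable threshold is met.
; Bait counts as in range once it reaches its impact point, regardless of position.
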(event Custom|ResetHitCount
  (Variables|Default|SetHitCount 0.0))

(event Custom|OnCatchBaitAnimationFinished
  (Default|CallOnReachSafeZone)
  (CallFunction|ResetHitCount))

(event EventOnCatchBait
  (params (Bait :type BP%20Bait%20Object%20Reference))
  (|CallParentFunction Bait)
  (bind _returnvalue (Utilities|Time|SetTimerbyEvent (delegate Custom|OnCatchBaitAnimationFinished) (Variables|Parameters|GetTimeBeforeBeingSafe)))
  (Variables|Default|SetCatchBaitTimer _returnvalue))

(fn ConstructionScript
  (|CallParentFunction))

(fn CanbeReeled
  (return (>= (Variables|Default|GetHitCount) (Variables|Parameters|GetHarpoonableHitCount))))

(fn OnHarpooned
  (Math|Float|IncrementFloat (Variables|Default|GetHitCount)
    (:%20%20
      (bind _canbereeled (CallFunction|CanbeReeled))
      (if _canbereeled
        (bind _success (|CallParentFunction))
        (if (and _success false)
          (Utilities|Time|ClearandInvalidateTimerbyHandle (Variables|Default|GetCatchBaitTimer))
          (return false false))))))

(fn IsBaitinRange
  (params (BaitPosition :type Vector :default "0, 0, 0") (HasReachedImpactPoint :type Boolean))
  (return HasReachedImpactPoint))