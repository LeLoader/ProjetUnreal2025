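; AI controller for a jumping fish that decides whether bait is in range by whether a launch arc can reach it.
; IsBaitInRange runs Unreal's projectile velocity suggestion from the pawn to the bait at a set launch speed, caching valid velocities for GetTossVelocity.
; The solve rotates both positions by the quaternion between world up and the negated target location, then unrotates the result.
; Debug drawing is left on.
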(event EventBeginPlay
  (|CallParentFunction) ; This node is disabled and will not be called.\nDrag off pins to build functionality.
)

(event EventTick
  (params (DeltaSeconds :type Float%20%28single-precision%29)))

(fn ConstructionScript
  (|CallParentFunction))

(fn SuggestProjectileVelocityCustomAngle
  (params (StartLocation :type Vector) (TargetLocation :type Vector) (LaunchSpeed :type Float%20%28double-precision%29))
  (bind _output_get (LocalVariables|SetRotationTargetToUp (Class|KismetMathLibrary|QuatFindBetweenVectors (Math|Vector|VectorUp) (Math|Vector|NegateVector TargetLocation))))
  (bind (_tossvelocity _returnvalue) (Class|GameplayStatics|BlueprintSuggestProjectileVelocity (Class|KismetMathLibrary|QuatRotateVector _output_get StartLocation) (Class|KismetMathLibrary|QuatRotateVector _output_get TargetLocation) LaunchSpeed 0.0 "DoNotTrace" 0.0 false true false))
  (return (Class|KismetMathLibrary|QuatUnrotateVector (LocalVariables|GetRotationTargetToUp) _tossvelocity) _returnvalue))

(fn IsBaitinRange
  (params (BaitPosition :type Vector :default "0, 0, 0"))
  (bind (_toss_velocity _valid) (CallFunction|SuggestProjectileVelocityCustomAngle (Transformation|GetActorLocation (Pawn|GetControlledPawn)) BaitPosition (Variables|Default|GetLaunchSpeed)))
  (if _valid
    (Variables|Default|SetTossVelocity _toss_velocity)
    (return true)
    (else
      (return false))))

(fn GetTossVelocity
  (return (Variables|Default|GetTossVelocity)))