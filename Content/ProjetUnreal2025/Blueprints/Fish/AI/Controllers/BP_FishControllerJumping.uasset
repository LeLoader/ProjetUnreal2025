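; AI controller for jumping fish that decides whether a bait is reachable by a leap and launches the fish at it.
; IsBaitInRange solves a toss velocity from the fish's jump and gravity strengths, storing it when valid for GetBait to apply as an impulse after Jump.
; The solver supports angled gravity by rotating positions with a quaternion built from the target's position vector, then unrotating the result, with debug drawing enabled.
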(event EventBeginPlay
  (|CallParentFunction))

(event EventTick
  (params (DeltaSeconds :type Float%20%28single-precision%29)))

(fn ConstructionScript
  (|CallParentFunction))

(fn SuggestProjectileVelocityCustomAngle
  (params (StartLocation :type Vector) (TargetLocation :type Vector) (LaunchSpeed :type Float%20%28double-precision%29) (Override%20Gravity :type Float%20%28double-precision%29))
  (bind _output_get (LocalVariables|SetRotationTargetToUp (Class|KismetMathLibrary|QuatFindBetweenVectors (Math|Vector|VectorUp) (Math|Vector|NegateVector TargetLocation))))
  (bind (_tossvelocity _returnvalue) (Class|GameplayStatics|BlueprintSuggestProjectileVelocity (Class|KismetMathLibrary|QuatRotateVector _output_get StartLocation) (Class|KismetMathLibrary|QuatRotateVector _output_get TargetLocation) LaunchSpeed (* Override%20Gravity -1e+02) "DoNotTrace" 0.0 false true false))
  (Rendering|Debug|DrawDebugArrow :LineStart StartLocation :LineEnd (+ (Class|KismetMathLibrary|QuatUnrotateVector (LocalVariables|GetRotationTargetToUp) _tossvelocity) StartLocation) :Duration 1.0)
  (return (Class|KismetMathLibrary|QuatUnrotateVector (LocalVariables|GetRotationTargetToUp) _tossvelocity) _returnvalue))

(fn IsBaitinRange
  (params (BaitPosition :type Vector :default "0, 0, 0") (Fish :type BP%20Fish%20Pawn%20Object%20Reference))
  (bind (_toss_velocity _valid) (CallFunction|SuggestProjectileVelocityCustomAngle (Transformation|GetActorLocation Fish) BaitPosition (Variables|/Game/ProjetUnreal2025/Blueprints/Fish/Pawns/BP_FishPawn.BP_FishPawn_C|GetJumpStrenght Fish) (Variables|/Game/ProjetUnreal2025/Blueprints/Fish/Pawns/BP_FishPawn.BP_FishPawn_C|GetGravityStrenght Fish)))
  (if _valid
    (Variables|Default|SetTossVelocity _toss_velocity)
    (return true)
    (else
      (return false))))

(fn GetBait
  (bind _asbp_fish_pawn (Utilities|Casting|CastToBP_FishPawn (Pawn|GetControlledPawn)))
  (Default|Jump _asbp_fish_pawn)
  (Physics|AddImpulse (Variables|/Game/ProjetUnreal2025/Blueprints/Fish/Pawns/BP_FishPawn.BP_FishPawn_C|GetRoot _asbp_fish_pawn) (Variables|Default|GetTossVelocity) "None" true)
  (return))