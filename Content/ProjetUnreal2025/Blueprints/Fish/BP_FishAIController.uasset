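; AI controller for fish that starts the BB_Fish blackboard and BT_Fish behavior tree on BeginPlay.
; When AI perception successfully senses a BP_Bait whose Sensed flag is false, it writes the bait's location to the SensedBait blackboard key.
; It then converts the stimulus tag to a bait enum and switches on it, but no case has any logic attached.
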(event OnTargetPerceptionUpdated(AIPerception)
  (params (Actor :type Actor%20Object%20Reference) (Stimulus :type AI%20Stimulus%20Structure))
  (bind (_age _expirationage _strength _stimuluslocation _receiverlocation _tag _bsuccessfullysensed) (Utilities|Struct|BreakAIStimulus Stimulus))
  (bind _asbp_bait (Utilities|Casting|CastToBP_Bait Actor))
  (if (and (not (Variables|/Game/ProjetUnreal2025/Blueprints/BP_Bait.BP_Bait_C|GetSensed _asbp_bait)) _bsuccessfullysensed)
    (AI|Components|Blackboard|SetValueasVector (stale EventBeginPlay _blackboardcomponent) (Utilities|Name|MakeLiteralName "SensedBait") (Transformation|GetActorLocation _asbp_bait))
    (switch Utilities|FlowControl|Switch|SwitchonE_Bait (Utilities|Enum|ByteToEnumE_Bait (Math|Conversions|ToByte(Integer) (Math|Conversions|ToInteger(Byte) (Utilities|String|ToString(Name) _tag)))))))

(event EventBeginPlay
  (bind _blackboardcomponent (Class|AIController|UseBlackboard "/Game/ProjetUnreal2025/Blueprints/Fish/AI/BB_Fish.BB_Fish"))
  (AI|RunBehaviorTree "/Game/ProjetUnreal2025/Blueprints/Fish/AI/BT_Fish.BT_Fish"))

(event EventTick
  (params (DeltaSeconds :type Float%20%28single-precision%29)))

(fn ConstructionScript)