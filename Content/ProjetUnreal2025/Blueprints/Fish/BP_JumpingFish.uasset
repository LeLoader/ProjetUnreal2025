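; BP_JumpingFish is a fish that leaps at bait when a valid ballistic arc can reach it.
; IsBaitInRange solves for a toss velocity, stores it and turns the fish toward the bait.
; The solver rotates positions by a quaternion from world up and the negated target position, applying custom gravity.
; CatchBait plays a sound, enables gravity, becomes harpoonable, sets the InAir blackboard key and launches via impulse.
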(event EventBeginPlay)

(event Collision|EventActorBeginOverlap
  (params (OtherActor :type Actor%20Object%20Reference)))

(event EventTick
  (params (DeltaSeconds :type Float%20%28single-precision%29))
  (|CallParentFunction DeltaSeconds) ; This node is disabled and will not be called.\nDrag off pins to build functionality.
)

(fn ConstructionScript
  (|CallParentFunction))

(fn SuggestProjectileVelocityCustomAngle
  (params (StartLocation :type Vector) (TargetLocation :type Vector) (LaunchSpeed :type Float%20%28double-precision%29) (CustomGravity :type Float%20%28double-precision%29))
  (bind _output_get (LocalVariables|SetRotationTargetToUp (Class|KismetMathLibrary|QuatFindBetweenVectors (Math|Vector|VectorUp) (Math|Vector|NegateVector TargetLocation))))
  (bind (_tossvelocity _returnvalue) (Class|GameplayStatics|BlueprintSuggestProjectileVelocity (Class|KismetMathLibrary|QuatRotateVector _output_get StartLocation) (Class|KismetMathLibrary|QuatRotateVector _output_get TargetLocation) LaunchSpeed (* CustomGravity -1e+02) "DoNotTrace" 0.0 false true false))
  (if _returnvalue
    (return (Class|KismetMathLibrary|QuatUnrotateVector (LocalVariables|GetRotationTargetToUp) _tossvelocity) true)
    (else
      (return "0, 0, 0" false))))

(fn CatchBait
  (params (Bait%20Location :type Vector :default "0, 0, 0"))
  (|CallParentFunction Bait%20Location)
  (Audio|PlaySoundatLocation (Variables|Default|GetJumpSound) (Transformation|GetActorLocation) "0, 0, 0" 1.0 1.0 0.0 0 0 0 0)
  (CallFunction|EnableGravity)
  (Variables|Default|SetHarpoonable true)
  (AI|Components|Blackboard|SetValueasBool (AI|GetBlackboard (AI|GetAIController self)) (Utilities|Name|MakeLiteralName "InAir") true)
  (CallFunction|Jump)
  (return))

(fn IsBaitinRange
  (params (Bait :type BP%20Bait%20Object%20Reference) (BaitLocation :type Vector :default "0, 0, 0") (HasReachedImpactPoint :type Boolean))
  (bind _returnvalue (Transformation|GetActorLocation))
  (bind (_toss_velocity _valid) (CallFunction|SuggestProjectileVelocityCustomAngle _returnvalue BaitLocation (Variables|Default|GetJumpStrenght) (Variables|Default|GetGravityStrenght)))
  (if _valid
    (Variables|Default|SetTossVelocity _toss_velocity)
    (Transformation|SetWorldRotation (Variables|Default|GetRoot) (Math|Rotator|FindLookatRotation _returnvalue BaitLocation) false false)
    (return true)
    (else
      (return false))))

(fn Jump
  (bind _root (Variables|Default|GetRoot))
  (bind _tossvelocity (Variables|Default|GetTossVelocity))
  (bind _returnvalue (Transformation|GetWorldLocation _root))
  (Physics|AddImpulse _root _tossvelocity "None" true)
  (Rendering|Debug|DrawDebugLine _returnvalue (+ _returnvalue _tossvelocity) "(R=1.000000,G=0.000000,B=0.957236,A=1.000000)" 1e+01 0.0))