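; Spherical bounds actor that spawns fish and manages their swim paths around the sphere.
; On play, it spawns configured counts per rarity from DT_Fishs with randomized size and weight, and replaces destroyed fish with the same rarity.
; Each fish gets a spline of random points on the radius plus offset, avoiding the poles, shifted forward as points are reached.
; Helpers supply center-pointing gravity and reroute splines toward a thrown bait's traced impact.
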(event Custom|SpawnRandomFish
  (bind _outrownames (DataTable|GetDataTableRowNames "/Game/ProjetUnreal2025/Data/DT_Fishs.DT_Fishs"))
  (CallFunction|SpawnFish (.OutItem (Utilities|Array|Random _outrownames))))

(event Custom|CreateBaseNavigationPoints
  (params (MovementComponent :type AC%20Fish%20Move%20Object%20Reference) (ZOffset :type Float%20%28double-precision%29))
  (bind _returnvalue (Components|GetOwner MovementComponent))
  (bind _tempposarray (Variables|Default|GetTempPosArray))
  (bind _returnvalue_2 (Transformation|GetActorLocation _returnvalue))
  (Utilities|Array|Add _tempposarray _returnvalue_2)
  (Utilities|Array|Add _tempposarray _returnvalue_2)
  (for _index (range 0 (- (Variables|Parameters|GetNavigationPointCount) 1))
    (Utilities|Array|Add (Variables|Default|GetTempPosArray) (CallFunction|GetCloseRandomPointinBounds (Variables|Parameters|GetZBoundsPercentage) (Utilities|GetLastIndex (Variables|Default|GetTempPosArray)) ZOffset 2e+01)))
  (Spline|SetSplinePoints (Variables|/Game/ProjetUnreal2025/Components/AC_FishMove.AC_FishMove_C|GetNavigationSpline MovementComponent) (Variables|Default|GetTempPosArray) "World" true)
  (Utilities|Array|Clear (Variables|Default|GetTempPosArray)))

(event Custom|RespawnFish
  (params (DestroyedActor :type Actor%20Object%20Reference))
  (bind _asbp_fish_pawn (Utilities|Casting|CastToBP_FishPawn DestroyedActor))
  (CallFunction|SpawnFishOfRarity (.rarity (Variables|/Game/ProjetUnreal2025/Blueprints/Fish/BP_FishPawn.BP_FishPawn_C|GetInfos _asbp_fish_pawn))))

(event Custom|OnFishSpawn
  (params (Fish :type BP%20Fish%20Pawn%20Object%20Reference))
  (bind _returnvalue (Actor|GetComponentbyClass Fish "/Game/ProjetUnreal2025/Components/AC_FishMove.AC_FishMove_C"))
  (Utilities|FlowControl|Sequence
    (:then_0
      (Utilities|IsValid _returnvalue
        (:Is%20Valid
          (bind _returnvalue_2 (Game|AddComponentbyClass "/Script/Engine.SplineComponent" true))
          (Variables|/Game/ProjetUnreal2025/Components/AC_FishMove.AC_FishMove_C|SetNavigationSpline _returnvalue _returnvalue_2)
          (CallFunction|CreateBaseNavigationPoints _returnvalue (Variables|/Game/ProjetUnreal2025/Components/AC_FishMove.AC_FishMove_C|GetZOffset _returnvalue)))))
    (:then_1
      (Game|BindEventtoOnDestroyed Fish (delegate Custom|RespawnFish)))))

(event Custom|OnReachedNavigationPoint
  (params (MoveComponent :type AC%20Fish%20Move%20Object%20Reference) (CreateNewPoint :type Boolean) (Angle :type Float%20%28double-precision%29) (ZOffset :type Float%20%28double-precision%29))
  (bind _tempposarray (Variables|Default|GetTempPosArray))
  (bind _navigationspline (Variables|/Game/ProjetUnreal2025/Components/AC_FishMove.AC_FishMove_C|GetNavigationSpline MoveComponent))
  ;[0.15 0.15 0.15 0.5] Delete 1st point, move each point down and recreate or not another point at the end
  (bind (_splinepoint _index) (Utilities|ForEachSplinePoint _navigationspline)
    (:LoopBody
      (if (not (== 0 _index))
        (Utilities|Array|Add (Variables|Default|GetTempPosArray) (.Position (Utilities|Struct|BreakSplinePoint _splinepoint)))))
    (:Completed
      (if CreateNewPoint
        (Utilities|Array|Add _tempposarray (CallFunction|GetCloseRandomPointinBounds (Variables|Parameters|GetZBoundsPercentage) (Utilities|GetLastIndex _tempposarray) ZOffset Angle)))
      (Spline|SetSplinePoints _navigationspline _tempposarray "World" true)
      (Utilities|Array|Clear _tempposarray))))

(event Custom|SpawnFish
  (params (Name :type Name))
  (bind _returnvalue (Math|Random|RandomFloat))
  (bind _returnvalue_2 (Utilities|GetDataTableRow "/Game/ProjetUnreal2025/Data/DT_Fishs.DT_Fishs" Name)
    (:then
      (if (.Spawnable (Utilities|Struct|BreakS_Fish _returnvalue_2))
        (bind _returnvalue_3 (Game|SpawnActorfromClass (.Class (Utilities|Struct|BreakS_Fish _returnvalue_2)) (Math|Transform|MakeTransform (CallFunction|GetRandomPointinBounds (Variables|Parameters|GetZBoundsPercentage)) "0, 0, 0" "1.000000,1.000000,1.000000") "AlwaysSpawn" "MultiplyWithRoot" 0 (.FavoriteBait (Utilities|Struct|BreakS_Fish _returnvalue_2)) 1.0 1.0 0))
        (CallFunction|OnFishSpawn _returnvalue_3)
        (Utilities|Struct|SetmembersinS_FishInfos (Variables|/Game/ProjetUnreal2025/Blueprints/Fish/BP_FishPawn.BP_FishPawn_C|GetInfos _returnvalue_3) (.Name (Utilities|Struct|BreakS_Fish _returnvalue_2)) (Math|Float|Lerp (.MinSize (Utilities|Struct|BreakS_Fish _returnvalue_2)) (.MaxSize (Utilities|Struct|BreakS_Fish _returnvalue_2)) _returnvalue) (Math|Float|Lerp (.MinWeight (Utilities|Struct|BreakS_Fish _returnvalue_2)) (.MaxWeight (Utilities|Struct|BreakS_Fish _returnvalue_2)) _returnvalue) (.Rarity (Utilities|Struct|BreakS_Fish _returnvalue_2)))
        (else
          (CallFunction|SpawnFishOfRarity (.Rarity (Utilities|Struct|BreakS_Fish _returnvalue_2))))))))

(event EventBeginPlay
  (bind _enumvalue (|ForEachE_Rarity)
    (:LoopBody
      (for _index (range 1 (.Value (Utilities|Map|Find (Variables|Parameters|GetFishPerRarity) _enumvalue)))
        (CallFunction|SpawnFishOfRarity _enumvalue)))))

(fn ConstructionScript
  (Components|Sphere|SetSphereRadius (Variables|Default|GetSphere) (Variables|Parameters|GetRadius) false))

(fn GetRandomPointinBounds
  (params (ZBoundsPercentage :type Float%20%28double-precision%29))
  (bind _returnvalue (* ZBoundsPercentage 2.0))
  (LocalVariables|SetRandomUnitVector (Math|Random|RandomUnitVector))
  (if (Math|Float|InRange(Float) (.Z (Math|Vector|BreakVector (LocalVariables|GetRandomUnitVector))) (+ _returnvalue -1.0) (- 1.0 _returnvalue))
    (return (+ (CallFunction|GetCenter) (* (CallFunction|GetRadius) (Math|Vector|MakeVector (.X (Math|Vector|BreakVector (LocalVariables|GetRandomUnitVector))) (.Y (Math|Vector|BreakVector (LocalVariables|GetRandomUnitVector))) (.Z (Math|Vector|BreakVector (LocalVariables|GetRandomUnitVector)))))))
    (else
      (return (CallFunction|GetRandomPointinBounds ZBoundsPercentage)))))

(fn GetCloseRandomPointinBounds
  (params (ZBoundsPercentage :type Float%20%28double-precision%29) (InitialPosition :type Vector) (FishZOffset :type Float%20%28double-precision%29) (Angle :type Float%20%28double-precision%29))
  (bind _returnvalue (* ZBoundsPercentage 2.0))
  (LocalVariables|SetRandomUnitVector (Math|Random|RandomUnitVectorinConeinDegrees (- InitialPosition (CallFunction|GetCenter)) Angle))
  (if (Math|Float|InRange(Float) (.Z (Math|Vector|BreakVector (LocalVariables|GetRandomUnitVector))) (+ _returnvalue -1.0) (- 1.0 _returnvalue))
    (return (+ (CallFunction|GetCenter) (* (+ (CallFunction|GetRadius) FishZOffset) (Math|Vector|MakeVector (.X (Math|Vector|BreakVector (LocalVariables|GetRandomUnitVector))) (.Y (Math|Vector|BreakVector (LocalVariables|GetRandomUnitVector))) (.Z (Math|Vector|BreakVector (LocalVariables|GetRandomUnitVector)))))))
    (else
      (return (CallFunction|GetCloseRandomPointinBounds ZBoundsPercentage InitialPosition FishZOffset 2e+01)))))

(fn GetCenter
  (return (Transformation|GetActorLocation)))

(fn GetGravityVector
  (params (ObjectPosition :type Vector))
  (return (* (Math|Vector|Normalize (- (CallFunction|GetCenter) ObjectPosition)) 9.81)))

(fn GetRadius
  (return (Components|Sphere|GetScaledSphereRadius (Variables|Default|GetSphere))))

(fn GetPointonSphere
  (params (Location :type Vector) (DistanceOffset :type Float%20%28double-precision%29))
  (return (* (Math|Vector|Normalize (- Location (CallFunction|GetCenter))) (+ DistanceOffset (CallFunction|GetRadius)))))

(fn RecalculateTrajectorytoBait
  (params (MovementComponent :type AC%20Fish%20Move%20Object%20Reference) (Bait :type BP%20Bait%20Object%20Reference) (DistanceOffset :type Float%20%28double-precision%29))
  (bind _returnvalue (Transformation|GetActorLocation Bait))
  (bind _returnvalue_2 (Components|GetOwner MovementComponent))
  (bind _navigationspline (Variables|/Game/ProjetUnreal2025/Components/AC_FishMove.AC_FishMove_C|GetNavigationSpline MovementComponent))
  (bind (_outhit _returnvalue_3) (Collision|LineTraceByChannel _returnvalue (+ _returnvalue (* (Math|Vector|Normalize (Variables|/Script/Engine.MovementComponent|GetVelocity (Variables|/Game/ProjetUnreal2025/Blueprints/BP_Bait.BP_Bait_C|GetThrowMovement Bait))) 1e+04)) "TraceTypeQuery1" false (Utilities|Array|MakeArray _returnvalue_2 Bait) "Persistent" false "(R=0.249492,G=1.000000,B=0.000000,A=1.000000)" "(R=0.000000,G=0.796659,B=1.000000,A=1.000000)" 1e+01))
  (if _returnvalue_3
    (Spline|SetSplinePoints _navigationspline (Utilities|Array|MakeArray (.Position (Utilities|Struct|BreakSplinePoint (Spline|GetSplinePointAt _navigationspline 1 "World"))) (Transformation|GetActorLocation _returnvalue_2) (+ (.ImpactPoint (Collision|BreakHitResult _outhit)) (* (Math|Vector|Normalize (- (.TraceStart (Collision|BreakHitResult _outhit)) (.TraceEnd (Collision|BreakHitResult _outhit)))) DistanceOffset))) "World" true))
  (return _returnvalue_3))

(fn SpawnFishOfRarity
  (params (Rarity :type E_Rarity%20Enum :default "NewEnumerator0"))
  (bind _possiblenames (LocalVariables|GetPossibleNames))
  (bind _outrownames (DataTable|GetDataTableRowNames "/Game/ProjetUnreal2025/Data/DT_Fishs.DT_Fishs"))
  (for _array_element _outrownames
    (bind _returnvalue (Utilities|GetDataTableRow "/Game/ProjetUnreal2025/Data/DT_Fishs.DT_Fishs" _array_element)
      (:then
        (if (Utilities|Enum|Equal(Enum) (.Rarity (Utilities|Struct|BreakS_Fish _returnvalue)) Rarity)
          (Utilities|Array|Add _possiblenames _array_element)))))
  (CallFunction|SpawnFish (.OutItem (Utilities|Array|Random _possiblenames))))