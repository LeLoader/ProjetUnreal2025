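; Base AI fish pawn that senses and eats bait, and can be harpooned and reeled into the player's catch.
; Sphere overlaps detect regular or favourite bait, feed it to the Blackboard and start a randomized eating timer on contact.
; Harpooning pauses eating and gravity; reeling hands the fish's info to the player and destroys it.
; When dropped, a radial force pulls it toward the world origin until an overlap restores its non-airborne state.
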(event OnComponentBeginOverlap(EatingZone)
  (params (OverlappedComponent :type Primitive%20Component%20Object%20Reference) (OtherActor :type Actor%20Object%20Reference) (OtherComp :type Primitive%20Component%20Object%20Reference) (OtherBodyIndex :type Integer) (bFromSweep :type Boolean) (SweepResult :type Hit%20Result%20Structure%20%28by%20ref%29))
  ;[0.15 0.15 0.15 0.5] Eating bait
  (bind _asbp_bait (Utilities|Casting|CastToBP_Bait OtherActor))
  (bind _output_get (Variables|Default|SetBait _asbp_bait))
  (CallFunction|OnCatchBait _output_get))

(event OnComponentBeginOverlap(FavouriteBaitDetection)
  (params (OverlappedComponent :type Primitive%20Component%20Object%20Reference) (OtherActor :type Actor%20Object%20Reference) (OtherComp :type Primitive%20Component%20Object%20Reference) (OtherBodyIndex :type Integer) (bFromSweep :type Boolean) (SweepResult :type Hit%20Result%20Structure%20%28by%20ref%29))
  (bind _asbp_bait (Utilities|Casting|CastToBP_Bait OtherActor))
  (if (Utilities|Enum|Equal(Enum) (Variables|/Game/ProjetUnreal2025/Blueprints/BP_Bait.BP_Bait_C|GetBaitType _asbp_bait) (Variables|Parameters|GetFavouriteBait))
    (CallFunction|BaitDetected _asbp_bait)))

(event OnComponentBeginOverlap(Root)
  (params (OverlappedComponent :type Primitive%20Component%20Object%20Reference) (OtherActor :type Actor%20Object%20Reference) (OtherComp :type Primitive%20Component%20Object%20Reference) (OtherBodyIndex :type Integer) (bFromSweep :type Boolean) (SweepResult :type Hit%20Result%20Structure%20%28by%20ref%29))
  (bind _returnvalue (Actor|GetComponentbyClass "/Game/ProjetUnreal2025/Components/AC_FishMove.AC_FishMove_C"))
  (Default|CallOnReachSafeZone)
  (CallFunction|DisableGravity)
  (Variables|Default|SetHarpoonable false)
  (AI|Components|Blackboard|SetValueasBool (AI|GetBlackboard (AI|GetAIController self)) (Utilities|Name|MakeLiteralName "InAir") false)
  (Utilities|IsValid _returnvalue
    (:Is%20Valid
      (Default|ResetDistance _returnvalue))))

(event OnComponentBeginOverlap(BaitDetection)
  (params (OverlappedComponent :type Primitive%20Component%20Object%20Reference) (OtherActor :type Actor%20Object%20Reference) (OtherComp :type Primitive%20Component%20Object%20Reference) (OtherBodyIndex :type Integer) (bFromSweep :type Boolean) (SweepResult :type Hit%20Result%20Structure%20%28by%20ref%29))
  (bind _asbp_bait (Utilities|Casting|CastToBP_Bait OtherActor))
  (CallFunction|BaitDetected _asbp_bait))

(event Custom|EnableGravity
  (Physics|SetSimulatePhysics (Variables|Default|GetRoot) true)
  (Variables|Default|SetIsGravityEnabled true))

(event Custom|DisableGravity
  (Physics|SetSimulatePhysics (Variables|Default|GetRoot) false)
  (Variables|Default|SetIsGravityEnabled false))

(event Custom|ClearTargetBait
  (params (DestroyedActor :type Actor%20Object%20Reference))
  ;[0.15 0.15 0.15 0.5] Eaten or destroyed by planet
  (Game|UnbindEventfromOnDestroyed DestroyedActor (delegate Custom|ClearTargetBait))
  (AI|Components|Blackboard|ClearValue (Variables|/Script/AIModule.AIController|GetBlackboard (AI|GetAIController self)) (Utilities|Name|MakeLiteralName "SensedBait"))
  (Utilities|Time|SetTimerbyEvent (delegate Custom|ReactivateCollision) (Variables|Parameters|GetTimeBeforeCollisionReactivation))
  (Default|CallOnTargetBaitGotDestroyed))

(event Custom|ReactivateCollision
  (Collision|SetCollisionEnabled (Variables|Default|GetBaitDetection) "QueryOnly")
  (Collision|SetCollisionEnabled (Variables|Default|GetFavouriteBaitDetection) "QueryOnly"))

(event Custom|EatBait
  (Actor|DestroyActor (Variables|Default|GetBait))
  (Variables|Default|SetBait 0))

(event Custom|DisableCollision
  (Collision|SetCollisionEnabled (Variables|Default|GetBaitDetection) "NoCollision")
  (Collision|SetCollisionEnabled (Variables|Default|GetFavouriteBaitDetection) "NoCollision"))

(event Custom|BaitDetected
  (params (Bait :type BP%20Bait%20Object%20Reference))
  (if (not (Variables|/Game/ProjetUnreal2025/Blueprints/BP_Bait.BP_Bait_C|GetSensed Bait))
    (Variables|/Game/ProjetUnreal2025/Blueprints/BP_Bait.BP_Bait_C|SetSensed Bait true)
    (Game|BindEventtoOnDestroyed Bait (delegate Custom|ClearTargetBait))
    (AI|Components|Blackboard|SetValueasObject (Variables|/Script/AIModule.AIController|GetBlackboard (AI|GetAIController self)) (Utilities|Name|MakeLiteralName "SensedBait") Bait)
    (CallFunction|DisableCollision)))

(event Custom|OnCatchBait
  (params (Bait :type BP%20Bait%20Object%20Reference))
  (Default|Eat Bait)
  (Transformation|AttachComponentToComponent Bait (Variables|Default|GetBaitSlot) "None" "SnapToTarget" "KeepWorld" "KeepWorld" true)
  (bind _returnvalue (Utilities|Time|SetTimerbyEvent (delegate Custom|EatBait) (+ (CallFunction|+- (Variables|Parameters|GetEatTime) (Variables|Parameters|GetEatTimeVariation)) 0.01)))
  (Variables|Default|SetEatingBaitTimer _returnvalue))

(event EventTick
  (params (DeltaSeconds :type Float%20%28single-precision%29))
  (Utilities|FlowControl|Sequence
    (:then_0
      (if (Variables|Parameters|GetUpdateRotation)
        (CallFunction|SetTargetRotation)
        (CallFunction|InterptoRotation DeltaSeconds)))
    (:then_1
      (if (Variables|Default|GetIsGravityEnabled)
        (Physics|AddRadialForce (Variables|Default|GetRoot) "0, 0, 0" 1e+05 (* (Variables|Parameters|GetGravityStrenght) -1e+02) "RIF_Constant" true)))))

(event EventOnDropped
  (AI|Components|Blackboard|SetValueasBool (AI|GetBlackboard (AI|GetAIController self)) (Utilities|Name|MakeLiteralName "IsHooked") false)
  (CallFunction|EnableGravity)
  (Transformation|DetachFromActor "KeepWorld" "KeepWorld" "KeepWorld")
  (Utilities|Time|UnpauseTimerbyHandle (Variables|Default|GetEatingBaitTimer))
  (Variables|Default|SetHarpoonable false)
  (AI|Components|Blackboard|SetValueasBool (AI|GetBlackboard (AI|GetAIController self)) (Utilities|Name|MakeLiteralName "InAir") true))

(event EventOnReeled
  (params (Player :type BP%20Fisherman%20Object%20Reference))
  (bind _infos (Variables|Default|GetInfos))
  (bind (_name _size _weight) (Utilities|Struct|BreakS_FishInfos _infos))
  (Utilities|Time|ClearandInvalidateTimerbyHandle (Variables|Default|GetEatingBaitTimer))
  ;[1 0 0.007892 0.5] Mettre dans la boite
  (Actor|DestroyActor (Variables|Default|GetBait))
  ;[1 0 0 0.5] REMOVE
  (Actor|DestroyActor)
  (Default|PutFish Player _infos)
  (Development|PrintText (Utilities|Text|FormatText (Class|KismetTextLibrary|MakeInvariantText "Fish is {0}, size of {1} and weight of {2}") _name _size _weight)))

(fn ConstructionScript
  (Components|Sphere|SetSphereRadius (Variables|Default|GetBaitDetection) (* (Variables|Parameters|GetBaitRange) 1e+02) false)
  (Components|Sphere|SetSphereRadius (Variables|Default|GetFavouriteBaitDetection) (* (Variables|Parameters|GetFavouriteBaitRange) 1e+02) false)
  (Components|Sphere|SetSphereRadius (Variables|Default|GetEatingZone) (* (Variables|Parameters|GetEatingRange) 1e+02) false))

(fn IsBaitinRange
  (params (BaitPosition :type Vector :default "0, 0, 0") (HasReachedImpactPoint :type Boolean))
  (return true))

(fn CatchBait
  (params (Bait%20Location :type Vector))
  (Variables|Default|SetHarpoonable true)
  (Components|Animation|PlayAnimation (Variables|Default|GetBody) (Variables|Parameters|GetGetBaitAnimation) false)
  (return))

(fn SetTargetRotation)

(fn InterptoRotation
  (params (Delta%20Seconds :type Float%20%28double-precision%29))
  (Transformation|SetActorRotation (Math|Interpolation|RInterpTo (Transformation|GetActorRotation) (Variables|Default|GetTargetRotation) Delta%20Seconds (Variables|Parameters|GetRotationSpeed))))

(fn CanbeReeled
  (return (Variables|Default|GetHarpoonable)))

(fn OnHarpooned
  (if (Variables|Default|GetHarpoonable)
    (AI|Components|Blackboard|SetValueasBool (AI|GetBlackboard (AI|GetAIController self)) (Utilities|Name|MakeLiteralName "IsHooked") true)
    (Utilities|Time|PauseTimerbyHandle (Variables|Default|GetEatingBaitTimer))
    (CallFunction|DisableGravity))
  (return (Variables|Default|GetHarpoonable) true))