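; BP_Rayquinox is a harpoonable fish that must be flipped onto its back before it can be caught.
; The first harpoon hit only sets OnBack and reports failure, while later hits defer to the parent's harpoon logic.
; Its target rotation follows velocity under gravity, otherwise the navigation spline tangent, with up taken radially from the world origin and inverted when on its back.
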(event EventBeginPlay)

(event Collision|EventActorBeginOverlap
  (params (OtherActor :type Actor%20Object%20Reference)))

(event EventTick
  (params (DeltaSeconds :type Float%20%28single-precision%29))
  (|CallParentFunction DeltaSeconds) ; This node is disabled and will not be called.\nDrag off pins to build functionality.
)

(fn ConstructionScript
  (|CallParentFunction))

(fn OnHarpooned
  (if (Variables|Default|GetOnBack)
    (bind (_success _manualreel) (|CallParentFunction))
    (return _success _manualreel)
    (else
      (Variables|Default|SetOnBack true)
      (return false false))))

(fn SetTargetRotation
  (bind _returnvalue (Transformation|GetActorLocation))
  (if (Variables|Default|GetIsGravityEnabled)
    (bind _returnvalue_2 (Physics|GetPhysicsLinearVelocity (Variables|Default|GetRoot) "None"))
    (return (Math|Rotator|MakeRotfromX _returnvalue_2))
    (else
      (return (Math|Rotator|MakeRotfromXZ (Spline|GetTangentatDistanceAlongSpline (Variables|Default|GetNavigationSpline) (CallFunction|GetDistancewithOffset) "Local") (Math|Vector|SelectVector (Math|Vector|NegateVector _returnvalue) _returnvalue (Variables|Default|GetOnBack)))))))