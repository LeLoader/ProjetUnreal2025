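; Kraky, a child fish Blueprint with tentacles that must be harpooned several times before it can be reeled in.
; At its path's end it waits for bait, magnetizes it to a tentacle socket and starts a timer that resumes roaming and resets hits.
; Harpooning cancels that timer and, while waiting, counts hits toward the reel threshold.
; Rotation faces world origin when harpooned, otherwise follows velocity or spline tangent with radial up.
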(event OnComponentBeginOverlap(BaitDetection)
  (params (OverlappedComponent :type Primitive%20Component%20Object%20Reference) (OtherActor :type Actor%20Object%20Reference) (OtherComp :type Primitive%20Component%20Object%20Reference) (OtherBodyIndex :type Integer) (bFromSweep :type Boolean) (SweepResult :type Hit%20Result%20Structure%20%28by%20ref%29))
  (AddComponent|AddACMagnetized OtherActor (Variables|Default|GetBody) "tentacle_bait_Socket" 1e+01)
  (bind _returnvalue (Utilities|Time|SetTimerbyEvent (delegate Custom|OnSafe) (Variables|Default|GetTimeBeforeBeingSafe)))
  (Variables|Default|SetSafeTimer _returnvalue)
  (Variables|Default|SetBaitInRange true))

(event Custom|OnReachLastPoint
  (Variables|Default|SetWaitingForBait true))

(event Custom|OnSafe
  (Default|CallKeepRoaming)
  (CallFunction|ResetHitCount))

(event Custom|Hit
  (Animation|Montage|PlayMontage (Variables|Default|GetBody) "/Game/ProjetUnreal2025/Art/Fishes/Fish02/anim/AM_KrakyHitTentacle.AM_KrakyHitTentacle"))

(event EventClearBaits
  (|CallParentFunction)
  (Variables|Default|SetWaitingForBait false)
  (Variables|Default|SetBaitInRange false))

(fn ConstructionScript
  (|CallParentFunction))

(fn SetTargetRotation
  (bind _returnvalue (Transformation|GetActorLocation))
  (bind _ac_fishmove (Variables|Components|GetAC_FishMove))
  (|CallParentFunction)
  (bind _returnvalue_2 (Physics|GetPhysicsLinearVelocity (Variables|Default|GetRoot) "None"))
  (Variables|Default|SetTargetRotation (Math|Rotator|SelectRotator (Math|Rotator|FindLookatRotation (Transformation|GetActorLocation) (Math|Vector|MakeVector 0.0 0.0 0.0)) (Math|Rotator|SelectRotator (Math|Rotator|MakeRotfromXZ _returnvalue_2 _returnvalue) (Math|Rotator|MakeRotfromXZ (Spline|GetTangentatDistanceAlongSpline (Variables|/Game/ProjetUnreal2025/Components/AC_FishMove.AC_FishMove_C|GetNavigationSpline _ac_fishmove) (Default|GetDistancewithOffset _ac_fishmove) "World") _returnvalue) (Variables|Default|GetIsGravityEnabled)) (Variables|Default|GetIsHarpooned))))

(fn RegisterMovementComponent
  (params (MovementComponent :type AC%20Fish%20Move%20Object%20Reference))
  (|CallParentFunction MovementComponent)
  (EventDispatchers|BindEventtoOnReachedLastPoint MovementComponent (EventDispatchers|CreateEvent :!event Custom|OnReachLastPoint)))

(fn IsBaitinRange
  (params (Bait :type BP%20Bait%20Object%20Reference) (BaitLocation :type Vector :default "0, 0, 0") (HasReachedImpactPoint :type Boolean))
  (bind _output_get (Variables|Default|SetWaitingForBait HasReachedImpactPoint))
  (return _output_get))

(fn OnHarpooned
  (if (Variables|Default|GetWaitingForBait)
    (bind _result (Math|Float|IncrementFloat (Variables|Default|GetHitCount))
      (:%20%20
        (if (< _result (- (Variables|Default|GetHarpoonableHitCount) 1.0))
          (CallFunction|Hit)))))
  (bind (_success _manualreel) (|CallParentFunction))
  (Utilities|Time|ClearandInvalidateTimerbyHandle (Variables|Default|GetSafeTimer))
  (return _success _manualreel))

(fn CanbeReeled
  (bind _canbereeled (|CallParentFunction))
  (return (and _canbereeled (>= (Variables|Default|GetHitCount) (Variables|Default|GetHarpoonableHitCount)))))