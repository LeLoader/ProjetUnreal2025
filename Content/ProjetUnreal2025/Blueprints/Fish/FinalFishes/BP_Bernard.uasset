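; Bernard fish Blueprint, a child of a shared fish class, that must hold a bait in each hand before it can be reeled in.
; Caught baits are magnetized to the left, then right hand socket on the body, and filling both makes it harpoonable.
; Clearing baits resets both hands and the harpoonable state.
; It also ignores WorldStatic collision when dropped and only interpolates rotation while gravity is enabled.
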(event EventBeginPlay)

(event Collision|EventActorBeginOverlap
  (params (OtherActor :type Actor%20Object%20Reference)))

(event EventTick
  (params (DeltaSeconds :type Float%20%28single-precision%29))
  (|CallParentFunction DeltaSeconds))

(event EventOnDropped
  (|CallParentFunction)
  (Collision|SetCollisionResponsetoChannel (Variables|Default|GetRoot) "ECC_WorldStatic" "ECR_Ignore"))

(event EventOnCatchBait
  (params (Bait :type BP%20Bait%20Object%20Reference) (AttachToBaitSlot :type Boolean) (SlotName :type Name :default "None"))
  (|CallParentFunction Bait false "main_bait_Socket")
  (if (Variables|Default|GetLeftHandFull)
    (if (not (Variables|Default|GetRightHandFull))
      (Variables|Default|SetRightHandFull true)
      (AddComponent|AddACMagnetized Bait (Variables|Default|GetBody) "R_bait_Socket" 7.5)
      (Variables|Default|SetHarpoonable true))
    (else
      (Variables|Default|SetLeftHandFull true)
      (AddComponent|AddACMagnetized Bait (Variables|Default|GetBody) "L_bait_Socket" 7.5))))

(event EventClearBaits
  (Variables|Default|SetLeftHandFull false)
  (Variables|Default|SetRightHandFull false)
  (Variables|Default|SetHarpoonable false)
  (|CallParentFunction))

(fn ConstructionScript
  (|CallParentFunction))

(fn CanbeReeled
  (bind _canbereeled (|CallParentFunction))
  (return (and _canbereeled (and (Variables|Default|GetLeftHandFull) (Variables|Default|GetRightHandFull)))))

(fn SetTargetRotation
  (bind _newtargetrotation (|CallParentFunction))
  (return _newtargetrotation))

(fn InterptoRotation
  (params (Delta%20Seconds :type Float%20%28double-precision%29))
  (if (Variables|Default|GetIsGravityEnabled)
    (|CallParentFunction Delta%20Seconds)))