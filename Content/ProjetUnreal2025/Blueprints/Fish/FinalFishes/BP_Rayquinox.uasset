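; Rayquinox fish Blueprint that can only be reeled in while flipped on its back.
; A harpoon hit when unreelable flips it and starts a timed recovery; dropping also clears the flip.
; Caught bait attaches to a socket as it keeps roaming, and range checks only require impact.
; Rotation faces world origin when harpooned, otherwise follows velocity under gravity or the spline tangent, using radial up from the origin.
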(event EventBeginPlay)

(event Collision|EventActorBeginOverlap
  (params (OtherActor :type Actor%20Object%20Reference)))

(event EventTick
  (params (DeltaSeconds :type Float%20%28single-precision%29))
  (|CallParentFunction DeltaSeconds) ; This node is disabled and will not be called.\nDrag off pins to build functionality.
)

(event EventOnCatchBait
  (params (Bait :type BP%20Bait%20Object%20Reference) (AttachToBaitSlot :type Boolean) (SlotName :type Name :default "None"))
  (|CallParentFunction Bait true "main_bait_Socket")
  (Default|CallKeepRoaming))

(event EventOnDropped
  (|CallParentFunction)
  (Variables|Default|SetOnBack false))

(fn ConstructionScript
  (|CallParentFunction))

(fn OnHarpooned
  (bind _canbereeled (CallFunction|CanbeReeled))
  (if _canbereeled
    (bind (_success _manualreel) (|CallParentFunction))
    (return _success _manualreel)
    (else
      (Variables|Default|SetHarpoonable true)
      (Variables|Default|SetOnBack true)
      (Utilities|Time|SetTimerbyEvent (EventDispatchers|CreateEvent :!event TurnBack) (Variables|Parameters|GetTimeBeforeTurningAgain))
      (return false false))))

(fn SetTargetRotation
  (bind _returnvalue (Transformation|GetActorLocation))
  (bind _ac_fishmove (Variables|Default|GetAC_FishMove))
  (|CallParentFunction)
  (bind _returnvalue_2 (Physics|GetPhysicsLinearVelocity (Variables|Default|GetRoot) "None"))
  (bind _output_get (Variables|Default|SetTargetRotation (Math|Rotator|SelectRotator (Math|Rotator|FindLookatRotation (Transformation|GetActorLocation) (Math|Vector|MakeVector 0.0 0.0 0.0)) (Math|Rotator|SelectRotator (Math|Rotator|MakeRotfromXZ _returnvalue_2 _returnvalue) (Math|Rotator|MakeRotfromZX _returnvalue (Spline|GetTangentatDistanceAlongSpline (Variables|/Game/ProjetUnreal2025/Components/AC_FishMove.AC_FishMove_C|GetNavigationSpline _ac_fishmove) (Default|GetDistancewithOffset _ac_fishmove) "World")) (Variables|Default|GetIsGravityEnabled)) (Variables|Default|GetIsHarpooned))))
  (return _output_get))

(fn TurnBack
  (Variables|Default|SetOnBack false))

(fn IsBaitinRange
  (params (Bait :type BP%20Bait%20Object%20Reference) (BaitLocation :type Vector :default "0, 0, 0") (HasReachedImpactPoint :type Boolean))
  (return HasReachedImpactPoint))

(fn CanbeReeled
  (bind _canbereeled (|CallParentFunction))
  (return (and _canbereeled (Variables|Default|GetOnBack))))