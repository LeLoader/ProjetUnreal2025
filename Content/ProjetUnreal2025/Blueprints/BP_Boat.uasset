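; Player boat that travels a looping spline around the planet, carrying the pawn and turning its view as the bearing to the planet center changes.
; Lever events play, stop or reverse a timeline that drives spline position, with motor sounds.
; The harpoon input context is added when stopped and removed when moving, with an arms toggle on each change.
; Three child-actor bait boxes report count changes per bait type and are refilled on load.
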(event Custom|CE_StartOrbit
  (Audio|PlaySound2D (Variables|Default|GetBoatSound) 1.0 1.0 0.0 0 0)
  (Components|Timeline|SetPlayRate (Variables|Default|GetTimeline) (/ 1.0 (Variables|Default|GetOrbitSpeed)))
  ;[0.15 0.15 0.15 0.5] Setting first rotation to prevent offset
  (Variables|Default|SetOldRotationAngle (Math|Rotator|FindLookatRotation (Transformation|GetActorLocation (Game|Player|GetPlayerPawn 0)) (Variables|/Game/ProjetUnreal2025/Blueprints/Global/GI_Fish.GI_Fish_C|GetPlanetCenter (Variables|Default|GetGI%20Fish))))
  (bind _returnvalue (Audio|SpawnSound2D (Variables|Default|GetMotorSound) 1.0 1.0 0.0 0 false false))
  (bind _output_get (Variables|Default|SetMotor _returnvalue))
  (Components|Activation|SetActive _output_get false false))

(event Custom|CE_PlayFromStart
  (Components|Activation|SetActive (Variables|Default|GetMotor) true false)
  (bind (_direction _float) (Timeline|Timeline PlayFromStart)
    (:Update
      (CallFunction|ChangeSelfandPawnPosition _float))
    (:Finished
      (switch Utilities|FlowControl|Switch|SwitchonETimelineDirection _direction
        (:Forward
          (CallFunction|CEPlayfromStart))
        (:Backward
          (CallFunction|CEReversefromEnd))))))

(event Custom|CE_Left
  (params (New%20Direction :type E_Movement%20Enum :default "NewEnumerator0"))
  (bind _returnvalue (Game|GetPlayerController 0))
  (bind _returnvalue_2 (PlayerController|LocalPlayerSubsystems|GetEnhancedInputLocalPlayerSubsystem _returnvalue))
  ;[0.15 0.15 0.15 0.5] Change Direction of timeline to suit lever changes
  (switch Utilities|FlowControl|Switch|SwitchonE_Movement New%20Direction
    (:NewEnumerator1
      (CallFunction|CEStop)
      (Audio|PlaySound2D (Variables|Default|GetMotorStopSound) 1.0 1.0 0.0 0 0)
      (Input|AddMappingContext _returnvalue_2 "/Game/ProjetUnreal2025/Inputs/IMC_Harpoon.IMC_Harpoon" 1 "(bIgnoreAllPressedKeysUntilRelease=True,bForceImmediately=False,bNotifyUserSettings=False)"))
    (:NewEnumerator2
      (CallFunction|CEReverse)
      (Audio|PlaySound2D (Variables|Default|GetMotorEntrySound) 1.0 1.0 0.0 0 0)
      (Input|RemoveMappingContext _returnvalue_2 "/Game/ProjetUnreal2025/Inputs/IMC_Harpoon.IMC_Harpoon" "(bIgnoreAllPressedKeysUntilRelease=True,bForceImmediately=False,bNotifyUserSettings=False)")))
  (Default|CallToggleArms))

(event Custom|CE_Play
  (Components|Activation|SetActive (Variables|Default|GetMotor) true false)
  (bind (_direction _float) (Timeline|Timeline Play)
    (:Update
      (CallFunction|ChangeSelfandPawnPosition _float))
    (:Finished
      (switch Utilities|FlowControl|Switch|SwitchonETimelineDirection _direction
        (:Forward
          (CallFunction|CEPlayfromStart))
        (:Backward
          (CallFunction|CEReversefromEnd))))))

(event Custom|CE_Reverse
  (Components|Activation|SetActive (Variables|Default|GetMotor) true false)
  (bind (_direction _float) (Timeline|Timeline Reverse)
    (:Update
      (CallFunction|ChangeSelfandPawnPosition _float))
    (:Finished
      (switch Utilities|FlowControl|Switch|SwitchonETimelineDirection _direction
        (:Forward
          (CallFunction|CEPlayfromStart))
        (:Backward
          (CallFunction|CEReversefromEnd))))))

(event Custom|CE_Right
  (params (NewDirection :type E_Movement%20Enum :default "NewEnumerator0"))
  (bind _returnvalue (Game|GetPlayerController 0))
  (bind _returnvalue_2 (PlayerController|LocalPlayerSubsystems|GetEnhancedInputLocalPlayerSubsystem _returnvalue))
  ;[0.15 0.15 0.15 0.5] Change Direction of timeline to suit lever changes
  (switch Utilities|FlowControl|Switch|SwitchonE_Movement NewDirection
    (:NewEnumerator0
      (CallFunction|CEPlay)
      (Audio|PlaySound2D (Variables|Default|GetMotorEntrySound) 1.0 1.0 0.0 0 0)
      (Input|RemoveMappingContext _returnvalue_2 "/Game/ProjetUnreal2025/Inputs/IMC_Harpoon.IMC_Harpoon" "(bIgnoreAllPressedKeysUntilRelease=True,bForceImmediately=False,bNotifyUserSettings=False)"))
    (:NewEnumerator1
      (CallFunction|CEStop)
      (Audio|PlaySound2D (Variables|Default|GetMotorStopSound) 1.0 1.0 0.0 0 0)
      (Input|AddMappingContext _returnvalue_2 "/Game/ProjetUnreal2025/Inputs/IMC_Harpoon.IMC_Harpoon" 1 "(bIgnoreAllPressedKeysUntilRelease=True,bForceImmediately=False,bNotifyUserSettings=False)")))
  (Default|CallToggleArms))

(event Custom|CE_ReverseFromEnd
  (Components|Activation|SetActive (Variables|Default|GetMotor) true false)
  (bind (_direction _float) (Timeline|Timeline ReverseFromEnd)
    (:Update
      (CallFunction|ChangeSelfandPawnPosition _float))
    (:Finished
      (switch Utilities|FlowControl|Switch|SwitchonETimelineDirection _direction
        (:Forward
          (CallFunction|CEPlayfromStart))
        (:Backward
          (CallFunction|CEReversefromEnd))))))

(event Custom|CE_Stop
  (Components|Activation|SetActive (Variables|Default|GetMotor) false false)
  (bind (_direction _float) (Timeline|Timeline Stop)
    (:Update
      (CallFunction|ChangeSelfandPawnPosition _float))
    (:Finished
      (switch Utilities|FlowControl|Switch|SwitchonETimelineDirection _direction
        (:Forward
          (CallFunction|CEPlayfromStart))
        (:Backward
          (CallFunction|CEReversefromEnd))))))

(event EventBeginPlay
  (Development|PrintString (Utilities|String|Append "location" (Utilities|String|ToString(Vector) (Transformation|GetActorLocation))) true true "(R=0.000000,G=0.660000,B=1.000000,A=1.000000)" 2e+01)
  (bind _asgi_fish (Utilities|Casting|CastToGI_Fish (Game|GetGameInstance)))
  (Variables|Default|SetGI%20Fish _asgi_fish)
  ;[0.15 0.15 0.15 0.5] Reacting To lever changes
  (bind _asbp_lever (Utilities|Casting|CastToBP_Lever (Variables|/Script/Engine.ChildActorComponent|GetChildActor (Variables|Default|GetLever))))
  (EventDispatchers|BindEventtoCallLeft _asbp_lever (EventDispatchers|CreateEvent :!event Custom|CE_Left))
  (EventDispatchers|BindEventtoCallRight _asbp_lever (EventDispatchers|CreateEvent :!event Custom|CE_Right))
  (Utilities|FlowControl|Sequence
    (:then_0
      (bind _asbp_bait_box (Utilities|Casting|CastToBP_BaitBox (Variables|/Script/Engine.ChildActorComponent|GetChildActor (Variables|Default|GetSomaliteBox))))
      (EventDispatchers|BindEventtoChangingNumber _asbp_bait_box (EventDispatchers|CreateEvent :!event ChangeSomaliteNumber)))
    (:then_1
      (bind _asbp_bait_box_2 (Utilities|Casting|CastToBP_BaitBox (Variables|/Script/Engine.ChildActorComponent|GetChildActor (Variables|Default|GetGlugmaliteBox))))
      (EventDispatchers|BindEventtoChangingNumber _asbp_bait_box_2 (EventDispatchers|CreateEvent :!event ChangeGlugmaliteNumber)))
    (:then_2
      (bind _asbp_bait_box_3 (Utilities|Casting|CastToBP_BaitBox (Variables|/Script/Engine.ChildActorComponent|GetChildActor (Variables|Default|GetMethaciteBox))))
      (EventDispatchers|BindEventtoChangingNumber _asbp_bait_box_3 (EventDispatchers|CreateEvent :!event ChangeMethaciteNumber)))))

(fn ConstructionScript)

(fn PutBaitinBox
  (params (BaitType :type E_Bait%20Enum :default "NewEnumerator0"))
  (bind _asbp_bait_box (Utilities|Casting|CastToBP_BaitBox (Variables|/Script/Engine.ChildActorComponent|GetChildActor (Utilities|Select :Index BaitType :NewEnumerator0 (Variables|Default|GetSomaliteBox) :NewEnumerator1 (Variables|Default|GetGlugmaliteBox) :NewEnumerator2 (Variables|Default|GetMethaciteBox)))))
  (bind _didput (Default|PutBait _asbp_bait_box))
  (return _didput))

(fn ChangeSomaliteNumber
  (params (Adding :type Boolean))
  (bind _somalitebaitnumber (Variables|Default|GetSomaliteBaitNumber))
  (if Adding
    (Math|Integer|IncrementInt _somalitebaitnumber)
    (else
      (Math|Integer|DecrementInt _somalitebaitnumber))))

(fn ChangeGlugmaliteNumber
  (params (Adding :type Boolean))
  (bind _glugmalitebaitnumber (Variables|Default|GetGlugmaliteBaitNumber))
  (if Adding
    (Math|Integer|IncrementInt _glugmalitebaitnumber)
    (else
      (Math|Integer|DecrementInt _glugmalitebaitnumber))))

(fn ChangeMethaciteNumber
  (params (Adding :type Boolean))
  (bind _methacitebaitnumber (Variables|Default|GetMethaciteBaitNumber))
  (if Adding
    (Math|Integer|IncrementInt _methacitebaitnumber)
    (else
      (Math|Integer|DecrementInt _methacitebaitnumber))))

(fn ChangeSelfandPawnPosition
  (params (Alpha :type Float%20%28double-precision%29))
  (bind _returnvalue (Game|Player|GetPlayerPawn 0))
  (bind _returnvalue_2 (Game|GetPlayerController 0))
  (bind _gi_fish (Variables|Default|GetGI%20Fish))
  (bind _spline (Variables|Default|GetSpline))
  (bind _returnvalue_3 (Transformation|GetActorLocation _returnvalue))
  (bind _returnvalue_4 (Spline|GetSplineLength _spline))
  (bind _planetcenter (Variables|/Game/ProjetUnreal2025/Blueprints/Global/GI_Fish.GI_Fish_C|GetPlanetCenter _gi_fish))
  (bind _returnvalue_5 (Math|Rotator|FindLookatRotation _returnvalue_3 _planetcenter))
  (bind _returnvalue_6 (Math|Float|Lerp 0.0 _returnvalue_4 Alpha))
  (bind _returnvalue_7 (Spline|GetTransformatDistanceAlongSpline _spline _returnvalue_6 "World" false))
  (Transformation|SetActorLocation _returnvalue (.location _returnvalue_7) false false)
  (Class|PlayerController|AddYawInput _returnvalue_2 (/ (.Yaw (Math|Rotator|BreakRotator (Math|Rotator|Delta(Rotator) _returnvalue_5 (Variables|Default|GetOldRotationAngle)))) (Class|PlayerController|GetDeprecatedInputYawScale _returnvalue_2)))
  (Variables|Default|SetOldRotationAngle _returnvalue_5)
  (Transformation|SetActorLocation (.location _returnvalue_7) false false)
  (Transformation|SetActorRotation _returnvalue_5))

(fn LoadBait
  (params (Somalite :type Integer) (Glugmalite :type Integer) (Methacite :type Integer))
  (Variables|Default|SetSomaliteBaitNumber Somalite)
  (Variables|Default|SetGlugmaliteBaitNumber Glugmalite)
  (Variables|Default|SetMethaciteBaitNumber Methacite)
  (Utilities|FlowControl|Sequence
    (:then_0
      (bind _asbp_bait_box (Utilities|Casting|CastToBP_BaitBox (Variables|/Script/Engine.ChildActorComponent|GetChildActor (Variables|Default|GetSomaliteBox))))
      (Default|PutBaitonLoad _asbp_bait_box (Variables|Default|GetSomaliteBaitNumber)))
    (:then_1
      (bind _asbp_bait_box_2 (Utilities|Casting|CastToBP_BaitBox (Variables|/Script/Engine.ChildActorComponent|GetChildActor (Variables|Default|GetGlugmaliteBox))))
      (Default|PutBaitonLoad _asbp_bait_box_2 (Variables|Default|GetGlugmaliteBaitNumber)))
    (:then_2
      (bind _asbp_bait_box_3 (Utilities|Casting|CastToBP_BaitBox (Variables|/Script/Engine.ChildActorComponent|GetChildActor (Variables|Default|GetMethaciteBox))))
      (Default|PutBaitonLoad _asbp_bait_box_3 (Variables|Default|GetMethaciteBaitNumber)))))