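; BP_Gravity is an actor that, once triggered, moves toward a gravity center point.
; It deactivates its GravityMovement component on BeginPlay until the CE_StartGraviting event activates it and sets the IsGraviting flag.
; While flagged, Tick overwrites the component's velocity with the direction to GravityCenter scaled by GravityStrength, giving constant-speed pull rather than acceleration, and prints debug messages.
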(event Custom|CE_StartGraviting
  (Variables|Default|SetIsGraviting true)
  (Components|Activation|Activate (Variables|Default|GetGravityMovement) false)
  (Development|PrintString "Started Graviting"))

(event EventBeginPlay
  (Components|Activation|Deactivate (Variables|Default|GetGravityMovement)))

(event EventTick
  (params (DeltaSeconds :type Float%20%28single-precision%29))
  (if (Variables|Default|GetIsGraviting)
    (Development|PrintString "Gravity Ticking")
    (Variables|/Script/Engine.MovementComponent|SetVelocity (Variables|Default|GetGravityMovement) (* (Math|Vector|Normalize (- (Variables|Default|GetGravityCenter) (Transformation|GetActorLocation))) (Variables|Default|GetGravityStrength)))))

(fn ConstructionScript)