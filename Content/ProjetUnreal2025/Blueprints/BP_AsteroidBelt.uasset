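; Asteroid belt actor that spawns debris and harpoonable bait along a spline and loops them around it each tick.
; BeginPlay redistributes the spline points evenly, fills all or selected segments by density, tops up bait, swaps in empty Bernard meteors and culls untracked attachments.
; Harpooned bait leaves a placeholder that respawns as bait after a cooldown.
; AttachBernardToRandom snaps a given Bernard onto a random unoccupied Bernard meteor.
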(event Custom|DivideSpline
  ;[0.15 0.15 0.15 0.5] Divide spline
  (for _index (range 0 (- (Variables|Spline|GetDivideSplineBy) 1))
    (bind _output_get (Variables|Spline|SetSplinePoint (* _index (Variables|Spline|GetSplineDividedLength))))
    (Utilities|Array|SetArrayElem (Variables|Spline|GetSplinePointsArray) _index _output_get true))
  (for _array_element (Variables|Spline|GetSplinePointsArray)
    (Utilities|Array|Add (Variables|Spline|GetSplinePointsLocations) (.location (Spline|GetTransformatDistanceAlongSpline (Variables|Default|GetSpline) _array_element "Local" false))))
  (Spline|ClearSplinePoints (Variables|Default|GetSpline) true)
  (for _array_element_2 (Variables|Spline|GetSplinePointsLocations)
    (Spline|AddSplinePoint (Variables|Default|GetSpline) _array_element_2 "Local" true)))

(event Custom|SpawnDebris
  (bind _returnvalue (Math|Random|RandomFloatinRange -1.8e+02 1.8e+02))
  ;[0.15 0.15 0.15 0.5] Spawn debris + bait
  (for _index (range 0 (- (Variables|Asteroids|GetSpawnCount) 1))
    (bind _output_get (Variables|Movement|SetMoveModifier (* _index (Variables|Asteroids|GetSpacing))))
    (if (Utilities|Array|IsEmpty (Variables|DivideSpline|GetArrayOfVectors))
      (Variables|Asteroids|SetSpawnLocation (.location (Spline|GetTransformatDistanceAlongSpline (Variables|Default|GetSpline) _output_get "World" false)) :!label _label)
      (Variables|Asteroids|SetSpawnRotation (Math|Rotator|MakeRotator _returnvalue _returnvalue _returnvalue))
      (if (> (Math|Random|RandomFloat) (/ (Variables|Bait|GetBaitConvertion) 1e+02))
        (bind _returnvalue_2 (Game|SpawnActorfromClass (.OutItem (Utilities|Array|Random (Variables|Asteroids|GetObjectsToSpawn))) (Math|Transform|MakeTransform (Variables|Asteroids|GetSpawnLocation) (Variables|Asteroids|GetSpawnRotation) (Math|Conversions|ToVector(Float) (Variables|Asteroids|GetObjectScale))) "DontSpawnIfColliding" "MultiplyWithRoot" 0 0))
        (Utilities|IsValid _returnvalue_2
          (:Is%20Valid
            (Transformation|AttachActorToActor _returnvalue_2 self "None" "KeepWorld" "KeepWorld" "KeepWorld" true)
            (Utilities|Array|Add (Variables|Movement|GetCurrentDistance) (Class|SplineComponent|GetDistanceAlongSplineatLocation (Variables|Default|GetSpline) (Transformation|GetActorLocation _returnvalue_2) "World"))))
        (else
          (Development|PrintString "aaaaaaaaaaaHello")
          (bind _returnvalue_3 (Game|SpawnActorfromClass (.OutItem (Utilities|Array|Random (Variables|Bait|GetBaitToSpawn))) (Math|Transform|MakeTransform (Variables|Asteroids|GetSpawnLocation) (Variables|Asteroids|GetSpawnRotation) (Math|Conversions|ToVector(Float) (Variables|Asteroids|GetObjectScale))) "DontSpawnIfColliding" "MultiplyWithRoot" 0 0))
          (Utilities|IsValid _returnvalue_3
            (:Is%20Valid
              (Transformation|AttachActorToActor _returnvalue_3 self "None" "KeepWorld" "KeepWorld" "KeepWorld" true)
              (EventDispatchers|BindEventtoHarpooned _returnvalue_3 (EventDispatchers|CreateEvent :!event Custom|CE_BaitHarpooned))
              (Development|PrintString "bound event to hit bait")
              (Utilities|Array|Add (Variables|Movement|GetCurrentDistance) (Class|SplineComponent|GetDistanceAlongSplineatLocation (Variables|Default|GetSpline) (Transformation|GetActorLocation) "World"))))))
      (else
        (for _array_element (Variables|DivideSpline|GetArrayOfVectors)
          (if (and (<= _output_get (.y _array_element)) (>= _output_get (.x _array_element)))
            (goto _label))))))
  (CallFunction|AddActorstoList)
  (CallFunction|VerifyifTheresBait)
  (CallFunction|SpawnBernardMeteor)
  (CallFunction|FindImmigrants))

(event Custom|SpawnBernard_Meteor
  (bind _allattachedobjects (Variables|Asteroids|GetAllAttachedObjects))
  (bind _returnvalue (Utilities|Array|LastIndex _allattachedobjects))
  (bind _returnvalue_2 (Math|Random|RandomIntegerinRange 0 _returnvalue))
  (bind _output (Utilities|Array|Get(acopy) _allattachedobjects _returnvalue_2))
  ;[0.15 0.15 0.15 0.5] B E R N A R D
  (for _index (range 0 (- (Variables|Bernard|GetAmountBernard_toSpawn) 1))
    (bind _returnvalue_3 (Game|SpawnActorfromClass "/Game/ProjetUnreal2025/Blueprints/Meteors/BP_Empty_Bernard.BP_Empty_Bernard_C" (Math|Transform|MakeTransform (Transformation|GetActorLocation _output) "0, 0, 0" (Math|Conversions|ToVector(Float) (Variables|Asteroids|GetObjectScale))) "AlwaysSpawn" "MultiplyWithRoot" 0 0))
    (Utilities|IsValid _output
      (:Is%20Valid
        (Actor|DestroyActor _output)
        (Transformation|AttachActorToActor _returnvalue_3 self "None" "KeepWorld" "KeepWorld" "KeepWorld" true)
        (Utilities|Array|SetArrayElem (Variables|Asteroids|GetAllAttachedObjects) _returnvalue_2 _returnvalue_3)))))

(event Custom|AddActorsToList
  ;[0.07588 0.08168 0.15 0.5] add all objects to list
  (Variables|Asteroids|SetAllAttachedObjects (Actor|GetAttachedActors self true false)))

(event Custom|DelayBeforeRespawn_Bait
  (params (RespawnableBait_Ref :type BP%20Respawnable%20Bait%20Object%20Reference))
  (bind _baittospawn (Variables|Bait|GetBaitToSpawn))
  ;[0.15 0.15 0.15 0.5] remove bait when harpooned
  (Utilities|FlowControl|Delay (Variables|Bait|GetBaitRespawnCooldown))
  (bind _returnvalue (Game|SpawnActorfromClass (Utilities|Array|Get(acopy) _baittospawn (Math|Random|RandomInteger (Utilities|Array|Length _baittospawn))) (Math|Transform|MakeTransform (Transformation|GetActorLocation RespawnableBait_Ref) "0, 0, 0" "1.000000,1.000000,1.000000") "AdjustIfPossibleButAlwaysSpawn" "MultiplyWithRoot" 0 0))
  (Transformation|AttachActorToActor _returnvalue self "None" "KeepWorld" "KeepWorld" "KeepWorld" true)
  (Utilities|Array|SetArrayElem (Variables|Asteroids|GetAllAttachedObjects) (Utilities|Array|FindItem (Variables|Asteroids|GetAllAttachedObjects) RespawnableBait_Ref) _returnvalue)
  (EventDispatchers|BindEventtoHarpooned _returnvalue (EventDispatchers|CreateEvent :!event Custom|CE_BaitHarpooned)))

(event Custom|CE_BaitHarpooned
  (params (Bait :type BP%20Bait%20Object%20Reference))
  ;[0.15 0.15 0.15 0.5] remove bait when harpooned
  (bind _returnvalue (Game|SpawnActorfromClass "/Game/ProjetUnreal2025/Blueprints/BP_RespawnableBait.BP_RespawnableBait_C" (Math|Transform|MakeTransform (Transformation|GetWorldLocation (Variables|/Game/ProjetUnreal2025/Blueprints/BP_Bait.BP_Bait_C|GetStaticMesh Bait)) "0, 0, 0" "1.000000,1.000000,1.000000") "AlwaysSpawn" "MultiplyWithRoot" 0 0))
  (Transformation|AttachActorToActor _returnvalue self "None" "KeepWorld" "KeepWorld" "KeepWorld" true)
  (Utilities|Array|SetArrayElem (Variables|Asteroids|GetAllAttachedObjects) (Utilities|Array|FindItem (Variables|Asteroids|GetAllAttachedObjects) Bait) _returnvalue)
  (CallFunction|DelayBeforeRespawnBait _returnvalue))

(event Custom|GetPointsToIgnore
  ;[0.15 0.15 0.15 0.5] set unique points to populate
  (for _array_element (Variables|DivideSpline|GetPointsToPopulate)
    (bind _output_get (Variables|DivideSpline|SetVectorToAdd (Math|Vector2D|MakeVector2D (Class|SplineComponent|GetDistanceAlongSplineatLocation (Variables|Default|GetSpline) (.location (Spline|GetTransformatSplinePoint (Variables|Default|GetSpline) _array_element "Local" false)) "Local") (+ (Class|SplineComponent|GetDistanceAlongSplineatLocation (Variables|Default|GetSpline) (.location (Spline|GetTransformatSplinePoint (Variables|Default|GetSpline) _array_element "Local" false)) "Local") (Variables|Spline|GetSplineDividedLength)))))
    (Utilities|Array|Add (Variables|DivideSpline|GetArrayOfVectors) _output_get)))

(event Custom|VerifyIfTheresBait
  (bind _baittospawn (Variables|Bait|GetBaitToSpawn))
  ;[0.15 0.15 0.15 0.5] Verify if there's bait in the "AllAttachedObjects" list
  (Variables|Bait|SetCurrentAmount_Bait 0)
  (bind _array_element (Utilities|Array|ForEachLoopwithBreak (Variables|Bait|GetBaitToSpawn) :!label _label)
    (:LoopBody
      (for _array_element_2 (Variables|Asteroids|GetAllAttachedObjects)
        (if (== (Utilities|GetClass _array_element_2) _array_element)
          (bind _output_get (Variables|Bait|SetCurrentAmount_Bait (+ (Variables|Bait|GetCurrentAmount_Bait) 1)))
          (if (>= _output_get (Variables|Bait|GetMinimumAmount_Bait))
            (Variables|Bait|SetIsThereBaits? (>= _output_get (Variables|Bait|GetMinimumAmount_Bait)))
            (goto _label Break)))))
    (:Completed
      (if (Variables|Bait|GetIsThereBaits?)
        (Development|PrintString "no need to spawn more baits")
        (else
          (for _index (range 0 (+ (- (Variables|Bait|GetMinimumAmount_Bait) (Variables|Bait|GetCurrentAmount_Bait)) 1))
            (bind _returnvalue (Game|SpawnActorfromClass (Utilities|Array|Get(acopy) _baittospawn (Math|Random|RandomInteger (Utilities|Array|Length _baittospawn))) (Math|Transform|MakeTransform (Transformation|GetActorLocation (Utilities|Array|Get(acopy) (Variables|Asteroids|GetAllAttachedObjects) (* _index 5))) "0, 0, 0" "1.000000,1.000000,1.000000") "AlwaysSpawn" "MultiplyWithRoot" 0 0))
            (Transformation|AttachActorToActor _returnvalue self "None" "KeepWorld" "KeepWorld" "KeepWorld" true)
            (Utilities|Array|SetArrayElem (Variables|Asteroids|GetAllAttachedObjects) (* _index 5) _returnvalue)
            (EventDispatchers|BindEventtoHarpooned _returnvalue (EventDispatchers|CreateEvent :!event Custom|CE_BaitHarpooned))))))))

(event Custom|FindImmigrants
  ;[0.15 0.15 0.15 0.5] FAITE LES PARTIIIIIIIIIIIR
  (for _array_element (Actor|GetAttachedActors true false)
    (if (== -1 (Utilities|Array|FindItem (Variables|Asteroids|GetAllAttachedObjects) _array_element))
      (Utilities|Array|Add (Variables|Default|GetItemsThatShouldntBe) _array_element)))
  (for _array_element_2 (Variables|Default|GetItemsThatShouldntBe)
    (Actor|DestroyActor _array_element_2)))

(event EventBeginPlay
  ;[0.05156 0.15 0.15 0.5] execution
  (bind _output_get (Variables|Spline|SetSplineLength (Spline|GetSplineLength (Variables|Default|GetSpline))))
  (Variables|Spline|SetSplineDividedLength (/ _output_get (Variables|Spline|GetDivideSplineBy)))
  (CallFunction|DivideSpline)
  (bind _output_get_2 (Variables|Asteroids|SetSpawnCount (Math|Float|Round (* (Variables|Spline|GetSplineLength) (Variables|Asteroids|GetSpawningDensity)))))
  (Variables|Asteroids|SetSpacing (/ (Variables|Spline|GetSplineLength) _output_get_2))
  (CallFunction|GetPointstoIgnore)
  (if (> (Variables|Asteroids|GetSpawnCount) 0)
    (CallFunction|SpawnDebris)))

(event EventTick
  (params (DeltaSeconds :type Float%20%28single-precision%29))
  ;[0.15 0.15 0.15 0.5] Move asteroids along spline
  (Variables|Movement|SetDistanceModifier (* DeltaSeconds (Variables|Movement|GetAsteroidMovespeed)))
  (for (_array_element _array_index) (Variables|Asteroids|GetAllAttachedObjects)
    (bind _output_get (Variables|Movement|SetNewDistanceR (+ (Variables|Movement|GetDistanceModifier) (Utilities|Array|Get(acopy) (Variables|Movement|GetCurrentDistance) _array_index))))
    (bind _output_get_2 (Variables|Movement|SetNewDistance (Math|Float|%(Float) _output_get (Spline|GetSplineLength (Variables|Default|GetSpline)))))
    (Utilities|Array|SetArrayElem (Variables|Movement|GetCurrentDistance) _array_index _output_get_2)
    (if (Utilities|IsValid _array_element)
      (Transformation|SetActorLocation _array_element (Spline|GetLocationatDistanceAlongSpline (Variables|Default|GetSpline) (Utilities|Array|Get(acopy) (Variables|Movement|GetCurrentDistance) _array_index) "World") false true))))

(fn ConstructionScript)

(fn AttachBernardtoRandom
  (params (Bernard :type Actor%20Object%20Reference))
  (bind _outactors (Actor|GetAllActorsOfClass "/Game/ProjetUnreal2025/Blueprints/Meteors/BP_Empty_Bernard.BP_Empty_Bernard_C"))
  (Utilities|Array|Shuffle _outactors)
  (bind _array_element (Utilities|Array|ForEachLoopwithBreak _outactors :!label _label)
    (:LoopBody
      (if (not (Variables|/Game/ProjetUnreal2025/Blueprints/Meteors/BP_Empty_Bernard.BP_Empty_Bernard_C|GetBernardInside _array_element))
        (Transformation|AttachActorToActor Bernard _array_element "None" "SnapToTarget" "KeepRelative" "KeepWorld" true)
        (Variables|/Game/ProjetUnreal2025/Blueprints/Meteors/BP_Empty_Bernard.BP_Empty_Bernard_C|SetBernardInside _array_element true)
        (LocalVariables|SetAttachedBernard true)
        (Game|BindEventtoOnDestroyed (EventDispatchers|CreateEvent _array_element :!event ClearBernardInside))
        (goto _label Break)))
    (:Completed
      (return (LocalVariables|GetAttachedBernard)))))