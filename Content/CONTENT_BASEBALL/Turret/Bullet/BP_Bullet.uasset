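; BP_Bullet is a turret projectile with support for being deflected by the player.
; DeflectingBullet turns it to a given rotation, relaunches it at InitialSpeed along local X and clears CanBeDeflectable.
; It also sets LaunchSpeed from a charge-based lerp, but the velocity call does not use it.
; Leaving the Sphere clears the flag for the first-person character, while the logic setting it true is disconnected.
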(event OnComponentBeginOverlap(Sphere)
  (params (OverlappedComponent :type Primitive%20Component%20Object%20Reference) (OtherActor :type Actor%20Object%20Reference) (OtherComp :type Primitive%20Component%20Object%20Reference) (OtherBodyIndex :type Integer) (bFromSweep :type Boolean) (SweepResult :type Hit%20Result%20Structure%20%28by%20ref%29)))

(event OnComponentEndOverlap(Sphere)
  (params (OverlappedComponent :type Primitive%20Component%20Object%20Reference) (OtherActor :type Actor%20Object%20Reference) (OtherComp :type Primitive%20Component%20Object%20Reference) (OtherBodyIndex :type Integer))
  (Utilities|Casting|CastToBP_FirstPersonCharacter OtherActor)
  (Variables|Default|SetCanBeDeflectable false)
  (Development|PrintString "Deflectable is FALSE"))

(event Custom|DeflectingBullet
  (params (LookRotation :type Rotator) (ChargeVal :type Float%20%28double-precision%29) (MinDeflectSpeed :type Float%20%28double-precision%29) (MaxDeflectSpeed :type Float%20%28double-precision%29))
  (bind _projectilemovement (Variables|Default|GetProjectileMovement))
  (Variables|Default|SetLaunchSpeed (Math|Float|Lerp MinDeflectSpeed MaxDeflectSpeed ChargeVal))
  (Transformation|SetActorRotation LookRotation)
  (Game|Components|ProjectileMovement|SetVelocityinLocalSpace _projectilemovement (Math|Vector|MakeVector (Variables|/Script/Engine.ProjectileMovementComponent|GetInitialSpeed _projectilemovement) 0.0 0.0))
  (Variables|Default|SetCanBeDeflectable false))

(fn ConstructionScript)